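; General AI character Blueprint that looks like a base class, with empty combat, death, stun, finisher and stealth assassination hooks.
; BeginPlay initializes the health widget from BPCStats and binds StartCombat to the player's chasing-tension event.
; Melee and arrow hits apply damage and report AI damage sense events, with arrows attaching to the nearest bone.
; Helpers handle time-dilation hit stop, ragdoll, arc jumps, injury recovery, and blackboard state and controller target queries.
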(event Custom|Ragdoll
  (Collision|SetCollisionEnabled (Variables|Character|GetMesh) "QueryAndPhysics")
  (Physics|SetSimulatePhysics (Variables|Character|GetMesh) true))

(event Custom|Die)

(event Custom|StartCombat)

(event EventBeginPlay
  (bind _aswb_enemy_health (Utilities|Casting|CastToWB_EnemyHealth (UserInterface|GetWidget (Variables|Default|GetEnemyStats))))
  (bind _output_get (Variables|UI|SetHealthUI _aswb_enemy_health))
  (bind _healthpercent (Default|GetCurrentHealth (Variables|Default|GetBPC_Stats)))
  (Progress|SetPercent (Variables|/Game/UI/WB_EnemyHealth.WB_EnemyHealth_C|GetHealthBar _output_get) _healthpercent)
  (bind _asbp_third_person_character (Utilities|Casting|CastToBP_ThirdPersonCharacter (Game|GetPlayerCharacter 0)))
  (bind _output_get_2 (Variables|General|SetPlayer _asbp_third_person_character))
  (EventDispatchers|BindEventtoOnChasingTension _output_get_2 (delegate Custom|StartCombat)))

(event Collision|EventActorBeginOverlap
  (params (OtherActor :type Actor%20Object%20Reference)))

(event EventMeleeDamage
  (params (Damage :type Float%20%28double-precision%29) (Attacker :type Pawn%20Object%20Reference))
  (bind _returnvalue (Game|Damage|ApplyDamage self Damage 0 0))
  (Class|AISenseDamage|ReportDamageEvent self Attacker _returnvalue (Transformation|GetActorLocation Attacker) "0, 0, 0" "None"))

(event EventStartHitStop
  (params (Duration :type Float%20%28double-precision%29))
  (Variables|Default|SetCustomTimeDilation 0.0)
  (Utilities|Time|SetTimerbyEvent (delegate EventEndHitStop) Duration))

(event EventEndHitStop
  (Variables|Default|SetCustomTimeDilation 1.0))

(event EventGetStunned)

(event EventFinisher)

(event EventTick
  (params (DeltaSeconds :type Float%20%28single-precision%29)))

(event EventEquipWeapon
  (params (Equipping? :type Boolean)))

(event EventArrowDamage
  (params (Damage :type Float%20%28double-precision%29) (Arrow :type BP%20Arrow%20Fly%20Object%20Reference) (HitLocation :type Vector :default "0, 0, 0") (Shooter :type Pawn%20Object%20Reference))
  (Transformation|AttachComponentToComponent Arrow (Variables|Character|GetMesh) (.ReturnValue (Class|SkinnedMeshComponent|FindClosestBoneK2 (Variables|Character|GetMesh) HitLocation 0.0)) "SnapToTarget" "KeepWorld" "KeepWorld" true)
  (bind _returnvalue (Game|Damage|ApplyDamage self Damage 0 0))
  (Class|AISenseDamage|ReportDamageEvent self Shooter _returnvalue (Transformation|GetActorLocation Shooter) "0, 0, 0" "None"))

(event EventSetState
  (params (newTension :type TensionEnum%20Enum :default "NewEnumerator0")))

(event EventSetMovementSpeed
  (params (Speed :type Float%20%28double-precision%29))
  (Variables|/Script/Engine.CharacterMovementComponent|SetMaxWalkSpeed (Variables|Character|GetCharacterMovement) Speed))

(event EventJumptoDestination
  (params (Destination :type Vector :default "0, 0, 0") (ZOffset :type Float%20%28double-precision%29) (GravityOverride :type Float%20%28double-precision%29) (ArcParam :type Float%20%28double-precision%29))
  (bind (_x _y _z) (Math|Vector|BreakVector Destination))
  (bind _outlaunchvelocity (Game|SuggestProjectileVelocityCustomArc (Transformation|GetActorLocation) (Math|Vector|MakeVector _x _y (+ _z ZOffset)) GravityOverride ArcParam))
  (Character|LaunchCharacter _outlaunchvelocity true true))

(fn ConstructionScript)

(fn CheckUpperBody
  (if (> (Math|Vector|VectorLength (Variables|/Script/Engine.MovementComponent|GetVelocity (Variables|Character|GetCharacterMovement))) 1e+02)
    (if (Variables|General|GetisInjured)
      (Variables|Movement|SetUpperBody false :!label _label)
      (else
        (Variables|Movement|SetUpperBody true)))
    (else
      (goto _label))))

(fn RunInjuredTimer
  (params (DeltaTime :type Float%20%28double-precision%29))
  (bind _bpc_stats (Variables|Default|GetBPC_Stats))
  (if (Variables|General|GetisInjured)
    (bind _output_get (Variables|General|SetinjuredTimer (+ (Variables|General|GetinjuredTimer) DeltaTime)))
    (if (>= _output_get (Variables|General|GetinjuredTimerMax))
      (Variables|General|SetisInjured false)
      (Variables|General|SetinjuredTimer 0.0)
      (Variables|Melee|SetisStunned false)
      (Variables|Default|SetisReceivingFinisher false)
      (Variables|/Game/ThirdPerson/Blueprints/BPC_Stats.BPC_Stats_C|SetStaminaRegenRate _bpc_stats 15.0)
      (Variables|/Game/ThirdPerson/Blueprints/BPC_Stats.BPC_Stats_C|SetpauseLoop _bpc_stats false))))

(fn Attack)

(fn GetCanMove
  (return (and (Variables|Movement|GetcanMove) (Variables|Melee|GetcanAttack))))

(fn GetGlobalTension
  (bind _asbp_third_person_character (Utilities|Casting|CastToBP_ThirdPersonCharacter (Game|GetPlayerCharacter 0)))
  (return (Variables|/Game/ThirdPerson/Blueprints/BP_ThirdPersonCharacter.BP_ThirdPersonCharacter_C|GettensionLevel _asbp_third_person_character)))

(fn GetIsInjured
  (return (Variables|General|GetisInjured)))

(fn GetPatrolRoute)

(fn GetState
  (return (Utilities|Enum|ByteToEnumTensionEnum (Class|BlackboardComponent|GetValueasEnum (AI|GetBlackboard (AI|GetAIController self)) (Utilities|Name|MakeLiteralName "State")))))

(fn GetStatus
  (return (Variables|/Game/ThirdPerson/Blueprints/BPC_Stats.BPC_Stats_C|GetisDead (Variables|Default|GetBPC_Stats))))

(fn GetTarget
  (bind _asbp_aicontroller_general (Utilities|Casting|CastToBP_AIController_General (Pawn|GetController)))
  (Utilities|IsValid (Variables|/Game/AI/BP_AIController_General.BP_AIController_General_C|GetattackTarget _asbp_aicontroller_general)
    (:Is%20Valid
      (return (Variables|/Game/AI/BP_AIController_General.BP_AIController_General_C|GetattackTarget _asbp_aicontroller_general)))))

(fn GetType
  (return "NewEnumerator0"))

(fn IsArmed
  (return false))

(fn IsDead
  (return (Variables|/Game/ThirdPerson/Blueprints/BPC_Stats.BPC_Stats_C|GetisDead (Variables|Default|GetBPC_Stats))))

(fn StealthAssassination)