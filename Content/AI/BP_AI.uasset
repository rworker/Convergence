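; Enemy AI character that plays as an axe Warrior or bow Archer, chosen by EnemyType, which spawns the matching weapon in construction.
; Warriors run combo montages with timer-driven sphere traces, while Archers draw, then fire arrows at the player via suggested projectile velocity.
; BPCStats drives a camera-facing health bar, hit reactions with knockback, and ragdoll death, including stealth assassination through a proximity prompt.
; Getters expose blackboard state, target and patrol route.
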(event OnComponentBeginOverlap(AssassinationRadius)
  (params (OverlappedComponent :type Primitive%20Component%20Object%20Reference) (OtherActor :type Actor%20Object%20Reference) (OtherComp :type Primitive%20Component%20Object%20Reference) (OtherBodyIndex :type Integer) (bFromSweep :type Boolean) (SweepResult :type Hit%20Result%20Structure%20%28by%20ref%29))
  (bind _isdead (Class|BPICombat|IsDead(Message) self))
  (if (not _isdead)
    (Utilities|Casting|CastToBP_ThirdPersonCharacter OtherActor)
    (Rendering|SetVisibility (Variables|Default|GetAssassinatePrompt) true false)))

(event OnComponentEndOverlap(AssassinationRadius)
  (params (OverlappedComponent :type Primitive%20Component%20Object%20Reference) (OtherActor :type Actor%20Object%20Reference) (OtherComp :type Primitive%20Component%20Object%20Reference) (OtherBodyIndex :type Integer))
  (Utilities|Casting|CastToBP_ThirdPersonCharacter OtherActor)
  (Rendering|SetVisibility (Variables|Default|GetAssassinatePrompt) false false))

(event Custom|Ragdoll
  (Collision|SetCollisionEnabled (Variables|Character|GetMesh) "QueryAndPhysics")
  (Physics|SetSimulatePhysics (Variables|Character|GetMesh) true))

(event Custom|ReceiveAssassination
  (Pawn|Components|CharacterMovement|DisableMovement (Variables|Character|GetCharacterMovement))
  (Class|NavMovementComponent|StopActiveMovement (Variables|Character|GetCharacterMovement))
  (Animation|Montage|PlayMontage (Variables|Character|GetMesh) "/Game/Characters/Mannequins/Animations/Quinn/Assassination/Paired_Knife_Stealth_KidneyAndNeck_Vic_Montage.Paired_Knife_Stealth_KidneyAndNeck_Vic_Montage"
    (:OnBlendOut
      (CallFunction|Die))
    (:OnNotifyBegin
      (bind _healthpercent (Default|InstaKill (Variables|Default|GetBPC_Stats)))
      (Progress|SetPercent (Variables|/Game/UI/WB_EnemyHealth.WB_EnemyHealth_C|GetHealthBar (Variables|Default|GetHealthUI)) _healthpercent))))

(event Custom|AttackInterrupted
  ;[0.05098 0.05098 0.05098] UseWeapon
  (switch Utilities|FlowControl|Switch|SwitchonEnemyEnum (Variables|Default|GetEnemyType)
    (:NewEnumerator0
      (CallFunction|StopCombo))
    (:NewEnumerator1
      (CallFunction|CancelShot))))

(event Custom|ResetSwordTrace
  (Utilities|FlowControl|DoOnce false) ; enters at Reset
)

(event Custom|ArrowSpawn
  ;[0.05098 0.05098 0.05098] SpawnArrow
  (Utilities|IsValid (Variables|Default|GetArrow)
    (:Is%20Not%20Valid
      (bind _returnvalue (Game|SpawnActorfromClass "/Game/Weapons/Arrow/BP_Arrow.BP_Arrow_C" (Transformation|GetWorldTransform (Variables|Character|GetMesh)) "Undefined" "MultiplyWithRoot" 0 self))
      (Variables|Default|SetArrow _returnvalue)
      (Transformation|AttachComponentToComponent (Variables|/Script/Engine.Actor|GetRootComponent _returnvalue) (Variables|Default|GetHandArrow) "None" "SnapToTarget" "SnapToTarget" "KeepWorld" true))))

(event Custom|CancelShot
  ;[0.05098 0.05098 0.05098] UseWeapon
  (Class|BPAnimInterface|SetAim(Message) (Components|SkeletalMesh|GetAnimInstance (Variables|Character|GetMesh)) false true)
  (Variables|Default|SetisPrimed false)
  (Variables|Default|SetisAiming false)
  (Default|CallOnFinishedAttackLocal)
  (Variables|Default|SetcanAttack true)
  (bind _arrow (Variables|Default|GetArrow)
    (:then
      (Actor|DestroyActor _arrow))
    (:else)))

(event Custom|LightAttack
  (bind _lightanims (Variables|Default|GetLightAnims))
  (bind _attackindex (Variables|Default|GetAttackIndex))
  (bind _output (Utilities|Array|Get(acopy) _lightanims _attackindex))
  ;[0.05098 0.05098 0.05098] SwordAttack
  (Utilities|FlowControl|DoOnce false :!label _label
    (:Completed
      (Utilities|FlowControl|Delay 0.1)
      (Variables|Default|SetattackAnimLength (Animation|GetPlayLength _output))
      (Animation|Montage|PlayMontage (Variables|Character|GetMesh) _output
        (:then
          (Math|Integer|IncrementInt (Variables|Default|GetAttackIndex)
            (:%20%20
              (goto _label Reset))))))))

(event Custom|StartSwordTrace
  (bind _returnvalue (Utilities|Time|SetTimerbyEvent (delegate Custom|SwordTraceLoop) 0.001 true))
  (Variables|Default|SetSwordTraceTimer _returnvalue))

(event Custom|SwordTraceLoop
  (bind _axeref (Variables|Default|GetAxeRef))
  (bind (_outhit _returnvalue) (Collision|SphereTraceByChannel (Transformation|GetWorldLocation (Variables|/Game/Weapons/Axe/BP_Axe.BP_Axe_C|GetBottom _axeref)) (Transformation|GetWorldLocation (Variables|/Game/Weapons/Axe/BP_Axe.BP_Axe_C|GetTop _axeref)) 12.0 "TraceTypeQuery1" false 0 "ForDuration" true "(R=1.000000,G=0.000000,B=0.000000,A=1.000000)" "(R=0.000000,G=1.000000,B=0.000000,A=1.000000)" 0.2))
  (if _returnvalue
    (if (Actor|ActorHasTag (.HitActor (Collision|BreakHitResult _outhit)) "Damageable")
      (Utilities|FlowControl|DoOnce false
        (:Completed
          (Niagara|SpawnSystematLocation "/Game/Weapons/Arrow/ArrowBloodBurst.ArrowBloodBurst" (.ImpactPoint (Collision|BreakHitResult _outhit)))
          (Game|Damage|ApplyDamage (.HitActor (Collision|BreakHitResult _outhit)) (Variables|Default|GetAttackDamage) 0 self))))))

(event Custom|Die
  (Default|CallEnemyDeath self)
  (Pawn|Components|CharacterMovement|DisableMovement (Variables|Character|GetCharacterMovement))
  (Class|BPICombat|SetState(Message) self "NewEnumerator0")
  (Rendering|SetVisibility (Variables|Default|GetHealthBar) false false)
  (CallFunction|Ragdoll)
  (Components|Activation|SetActive (Variables|Default|GetAssassination%20Radius) false false)
  (Collision|SetCollisionEnabled (Variables|Collision|GetCapsuleComponent) "NoCollision")
  (Components|DestroyComponent (Variables|Collision|GetCapsuleComponent)))

(event Custom|StopSwordTrace
  (Utilities|Time|ClearandInvalidateTimerbyHandle (Variables|Default|GetSwordTraceTimer))
  (CallFunction|ResetSwordTrace))

(event Custom|BowCall
  (bind _bowref (Variables|Default|GetBowRef))
  (bind _rootcomponent (Variables|/Script/Engine.Actor|GetRootComponent _bowref))
  (bind _returnvalue (Transformation|GetWorldLocation _rootcomponent))
  (bind _returnvalue_2 (Math|Vector|GetUpVector _rootcomponent))
  (bind _returnvalue_3 (* _returnvalue_2 1.0))
  (bind _returnvalue_4 (+ _returnvalue _returnvalue_3))
  ;[0.05098 0.05098 0.05098] UseWeapon
  (Utilities|FlowControl|Sequence
    (:then_0
      (if (Variables|Default|GetcanAttack)
        (Variables|Default|SetcanAttack false)
        (if (Variables|Default|GetcanAim)
          (Variables|Default|Setstrength 1e+03)
          (Variables|/Script/Engine.CharacterMovementComponent|SetMaxWalkSpeed (Variables|Character|GetCharacterMovement) 2e+02)
          (bind _output_get (Variables|Default|SetisAiming true))
          (bind _notifyname (Animation|Montage|PlayMontage (Variables|Character|GetMesh) "/Game/Characters/Mannequins/Animations/Quinn/Bow/BowAnimation/aim/StandingDrawArrow_UE_Montage1.StandingDrawArrow_UE_Montage1")
            (:OnBlendOut
              (Class|BPAnimInterface|SetAim(Message) (Components|SkeletalMesh|GetAnimInstance (Variables|Character|GetMesh)) _output_get false))
            (:OnNotifyBegin
              (if (== _notifyname "SpawnArrow")
                (CallFunction|ArrowSpawn)
                (elif (== _notifyname "Pull")
                  (Variables|Default|SetisPrimed true))))))))
    (:then_1
      (Utilities|FlowControl|Delay 3.0)
      (if (Variables|Default|GetisAiming)
        (Variables|/Script/Engine.CharacterMovementComponent|SetMaxWalkSpeed (Variables|Character|GetCharacterMovement) 3e+02)
        (bind _notifyname_2 (Animation|Montage|PlayMontage (Variables|Character|GetMesh) "/Game/Characters/Mannequins/Animations/Quinn/Bow/BowAnimation/Equip/StandingAimRecoil_UE_Montage.StandingAimRecoil_UE_Montage")
          (:OnBlendOut
            (Class|BPAnimInterface|SetAim(Message) (Components|SkeletalMesh|GetAnimInstance (Variables|Character|GetMesh)) false true)
            (Default|CallOnFinishedAttackLocal))
          (:OnNotifyBegin
            (if (== _notifyname_2 "Release")
              (bind _asactor (Utilities|Casting|CastToActor (Game|GetPlayerCharacter 0)))
              (bind _tossvelocity (Class|GameplayStatics|BlueprintSuggestProjectileVelocity _returnvalue_4 (Transformation|GetActorLocation _asactor) (Variables|Default|Getstrength) 0.0 "DoNotTrace" 0.0 false false))
              (Game|SpawnActorfromClass "/Game/Weapons/Arrow/BP_ArrowFly.BP_ArrowFly_C" (Math|Transform|MakeTransform _returnvalue_4 (Math|Rotator|MakeRotfromX _tossvelocity) "1.000000,1.000000,1.000000") "Undefined" "MultiplyWithRoot" 0 (Variables|Default|Getstrength) self)
              (Variables|Default|SetisPrimed false)
              (bind _arrow (Variables|Default|GetArrow)
                (:then
                  (Actor|DestroyActor _arrow)
                  (Variables|Default|SetcanAttack true))
                (:else)))))))))

(event Custom|MeleeCall
  ;[0.05098 0.05098 0.05098] SwordAttack
  (CallFunction|SwordAttack))

(event Custom|HeavyAttack
  ;[0.05098 0.05098 0.05098] SwordAttack
  (Utilities|FlowControl|DoOnce false :!label _label
    (:Completed
      (Utilities|FlowControl|Delay 0.1)
      (Animation|Montage|PlayMontage (Variables|Character|GetMesh) (Utilities|Array|Get(acopy) (Variables|Default|GetHeavyAnims) (Variables|Default|GetAttackIndex))
        (:then
          (Math|Integer|IncrementInt (Variables|Default|GetAttackIndex)
            (:%20%20
              (goto _label Reset))))))))

(event Custom|SwordAttack
  ;[0.05098 0.05098 0.05098] SwordAttack
  (if (Variables|Default|Getholding)
    (if (Variables|Default|GetisHeavy)
      _
      (else
        (Variables|Default|SetAttackIndex 0)
        (Variables|Default|SetisHeavy true)))
    (CallFunction|HeavyAttack)
    (else
      (if (Variables|Default|GetisHeavy)
        (Variables|Default|SetAttackIndex 0)
        (Variables|Default|SetisHeavy false))
      (CallFunction|LightAttack))))

(event Custom|SwordAttackCombo
  ;[0.05098 0.05098 0.05098] SwordAttack
  (if (Variables|Default|GetsaveAttack)
    (Variables|Default|SetsaveAttack false)
    (if (Variables|Default|Getholding)
      (if (Variables|Default|GetisHeavy)
        _
        (else
          (Variables|Default|SetAttackIndex 0)
          (Variables|Default|SetisHeavy true)))
      (CallFunction|HeavyAttack)
      (else
        (if (Variables|Default|GetisHeavy)
          (Variables|Default|SetAttackIndex 0)
          (Variables|Default|SetisHeavy false))
        (CallFunction|LightAttack)))))

(event Custom|StopCombo
  (bind _self self)
  ;[0.05098 0.05098 0.05098] SwordAttack
  (Variables|Default|SetisAttacking false)
  (Variables|Default|SetAttackIndex 0)
  (Variables|Default|SetisHeavy false)
  (Utilities|FlowControl|Delay 0.5)
  (Default|CallOnFinishedAttackLocal _self)
  (Default|CallOnFinishedAttackGlobal _self)
  (Animation|StopAnimMontage 0))

(event Input|EnhancedActionEvents|EnhancedInputActionIA_UseBow
  (params (ActionValue :type Boolean) (ElapsedSeconds :type Float%20%28double-precision%29) (TriggeredSeconds :type Float%20%28double-precision%29) (InputAction :type Input%20Action%20Object%20Reference :default "/Game/ThirdPerson/Input/Actions/IA_UseBow.IA_UseBow"))
  ;[0.05098 0.05098 0.05098] UseWeapon
)

(event EventBeginPlay
  (bind _aswb_enemy_health (Utilities|Casting|CastToWB_EnemyHealth (UserInterface|GetWidget (Variables|Default|GetHealthBar))))
  (bind _output_get (Variables|Default|SetHealthUI _aswb_enemy_health))
  (bind _healthpercent (Default|GetCurrentHealth (Variables|Default|GetBPC_Stats)))
  (Progress|SetPercent (Variables|/Game/UI/WB_EnemyHealth.WB_EnemyHealth_C|GetHealthBar _output_get) _healthpercent)
  (Class|BPAnimInterface|CheckEnemyType(Message) (Components|SkeletalMesh|GetAnimInstance (Variables|Character|GetMesh)) (Variables|Default|GetEnemyType))
  (Development|PrintString "Hello"))

(event Collision|EventActorBeginOverlap
  (params (OtherActor :type Actor%20Object%20Reference)))

(event EventMeleeDamage
  (params (Damage :type Float%20%28double-precision%29) (Attacker :type Pawn%20Object%20Reference))
  (bind _returnvalue (Game|Damage|ApplyDamage self Damage 0 0))
  (Class|AISenseDamage|ReportDamageEvent self Attacker _returnvalue (Transformation|GetActorLocation Attacker) "0, 0, 0" "None"))

(event EventTick
  (params (DeltaSeconds :type Float%20%28single-precision%29))
  (bind _returnvalue (AI|GetBlackboard 0))
  (bind _returnvalue_2 (Utilities|Name|MakeLiteralName "TargetActor"))
  (bind _returnvalue_3 (AI|Components|Blackboard|GetValueasObject _returnvalue _returnvalue_2))
  (Transformation|SetWorldRotation (Variables|Default|GetHealthBar) (Math|Rotator|FindLookatRotation (Transformation|GetWorldLocation (Variables|Default|GetHealthBar)) (Transformation|GetWorldLocation (Variables|/Script/Engine.PlayerCameraManager|GetTransformComponent (Game|GetPlayerCameraManager 0)))) false false)
  (CallFunction|CheckUpperBody)
  (CallFunction|RunInjuredTimer DeltaSeconds)
  (Utilities|IsValid _returnvalue_3
    (:Is%20Valid
      (bind _asactor (Utilities|Casting|CastToActor _returnvalue_3))
      (Class|BPAnimInterface|SetUpperBodyRotation(Message) (Components|SkeletalMesh|GetAnimInstance (Variables|Character|GetMesh)) (Math|Rotator|MakeRotator (- 3.6e+02 (.pitch (Math|Rotator|FindLookatRotation (Transformation|GetActorLocation) (Transformation|GetActorLocation _asactor)))) 0.0 0.0)))))

(event Game|Damage|EventAnyDamage
  (params (Damage :type Float%20%28single-precision%29) (DamageType :type Damage%20Type%20Object%20Reference) (InstigatedBy :type Controller%20Object%20Reference) (DamageCauser :type Actor%20Object%20Reference))
  (bind _healthbar (Variables|Default|GetHealthBar))
  (CallFunction|CancelShot)
  (Variables|Default|SetinjuredTimer 0.0)
  (Class|NavMovementComponent|StopActiveMovement (Variables|Character|GetCharacterMovement))
  (CallFunction|StopCombo)
  (if (not (Variables|/Game/ThirdPerson/Blueprints/BPC_Stats.BPC_Stats_C|GetisDead (Variables|Default|GetBPC_Stats)))
    (if (Variables|Default|GetisInjured)
      _
      (else
        (Variables|Default|SetisInjured true)
        (Animation|Montage|PlayMontage (Variables|Character|GetMesh) (Utilities|Array|Get(acopy) (Variables|Default|GethitAnims) (Math|Random|RandomIntegerinRange 0 (- (Utilities|Array|Length (Variables|Default|GethitAnims)) 1)))
          (:then
            _))))
    (bind _asbp_third_person_character (Utilities|Casting|CastToBP_ThirdPersonCharacter (Game|GetPlayerCharacter 0)))
    (Character|LaunchCharacter (* (Math|Vector|GetForwardVector (Transformation|GetActorRotation _asbp_third_person_character)) 7e+02) false false)
    (bind (_isdead _healthpercent) (Default|DecreaseHealth (Variables|Default|GetBPC_Stats) Damage))
    (if (Rendering|IsVisible _healthbar)
      _
      (else
        (Rendering|SetVisibility _healthbar true false)))
    (Progress|SetPercent (Variables|/Game/UI/WB_EnemyHealth.WB_EnemyHealth_C|GetHealthBar (Variables|Default|GetHealthUI)) _healthpercent)
    (if _isdead
      (Utilities|FlowControl|Delay 0.2)
      (CallFunction|Die))))

(event EventArrowDamage
  (params (Damage :type Float%20%28double-precision%29) (Arrow :type BP%20Arrow%20Fly%20Object%20Reference) (HitLocation :type Vector :default "0, 0, 0") (Shooter :type Pawn%20Object%20Reference))
  (Transformation|AttachComponentToComponent Arrow (Variables|Character|GetMesh) (.ReturnValue (Class|SkinnedMeshComponent|FindClosestBoneK2 (Variables|Character|GetMesh) HitLocation 0.0)) "SnapToTarget" "KeepWorld" "KeepWorld" true)
  (bind _returnvalue (Game|Damage|ApplyDamage self Damage 0 0))
  (Class|AISenseDamage|ReportDamageEvent self Shooter _returnvalue (Transformation|GetActorLocation Shooter) "0, 0, 0" "None"))

(event EventEquipWeapon
  (params (Equipping? :type Boolean))
  (bind _mesh (Variables|Character|GetMesh))
  (bind _mesh_2 (Variables|Character|GetMesh))
  (bind _enemytype (Variables|Default|GetEnemyType))
  (if Equipping?
    (switch Utilities|FlowControl|Switch|SwitchonEnemyEnum _enemytype
      (:NewEnumerator0
        (Animation|Montage|PlayMontage _mesh "/Game/Characters/Enemy/Warrior/Animations/Unarmed_Equip_Underarm_Anim_Montage.Unarmed_Equip_Underarm_Anim_Montage"
          (:OnInterrupted
            _)
          (:OnNotifyBegin
            _))
        (Transformation|AttachComponentToComponent (Variables|/Script/Engine.Actor|GetRootComponent (Variables|Default|GetAxeRef)) (Variables|Default|GetHandAxe) "None" "SnapToTarget" "SnapToTarget" "SnapToTarget" true))
      (:NewEnumerator1
        (Animation|Montage|PlayMontage _mesh "/Game/Characters/Mannequins/Animations/Quinn/Bow/BowAnimation/Equip/StandingEquipBow.StandingEquipBow"
          (:OnInterrupted
            _)
          (:OnNotifyBegin
            _))
        (Transformation|AttachComponentToComponent (Variables|/Script/Engine.Actor|GetRootComponent (Variables|Default|GetBowRef)) (Variables|Default|GetHandBow) "None" "SnapToTarget" "SnapToTarget" "SnapToTarget" true)))
    (Variables|Default|SetIsArmed_0 true)
    (Default|CallDoneEquipping)
    (else
      (switch Utilities|FlowControl|Switch|SwitchonEnemyEnum _enemytype
        (:NewEnumerator0
          (Animation|Montage|PlayMontage _mesh_2 "/Game/Characters/Enemy/Warrior/Animations/Standing_Disarm_Underarm_Anim_Montage.Standing_Disarm_Underarm_Anim_Montage"
            (:OnInterrupted
              _)
            (:OnNotifyBegin
              _))
          (Transformation|AttachComponentToComponent (Variables|/Script/Engine.Actor|GetRootComponent (Variables|Default|GetAxeRef)) (Variables|Default|GetBackAxe) "None" "SnapToTarget" "SnapToTarget" "SnapToTarget" true))
        (:NewEnumerator1
          (Animation|Montage|PlayMontage _mesh_2 "/Game/Characters/Mannequins/Animations/Quinn/Bow/BowAnimation/Equip/StandingDisarmBow_Idle.StandingDisarmBow_Idle"
            (:OnInterrupted
              _)
            (:OnNotifyBegin
              _))
          (Transformation|AttachComponentToComponent (Variables|/Script/Engine.Actor|GetRootComponent (Variables|Default|GetBowRef)) (Variables|Default|GetBackBow) "None" "SnapToTarget" "SnapToTarget" "SnapToTarget" true)))
      (Variables|Default|SetIsArmed_0 false)
      (Default|CallDoneEquipping))))

(event EventSetMovementSpeed
  (params (Speed :type Float%20%28double-precision%29))
  (bind _output_get (Variables|/Script/Engine.CharacterMovementComponent|SetMaxWalkSpeed (Variables|Character|GetCharacterMovement) Speed)))

(event EventSetState
  (params (newTension :type TensionEnum%20Enum :default "NewEnumerator0"))
  (AI|Components|Blackboard|SetValueasEnum (AI|GetBlackboard (AI|GetAIController self)) (Utilities|Name|MakeLiteralName "State") newTension)
  (Default|CallUpdatedTension newTension))

(event EventLookIdle
  (Animation|Montage|PlayMontage (Variables|Character|GetMesh) "/Game/Characters/Enemy/Warrior/Animations/Sword_And_Shield_Idle__1__Montage.Sword_And_Shield_Idle__1__Montage"))

(event EventWaitIdle
  (Animation|Montage|PlayMontage (Variables|Character|GetMesh) "/Game/Characters/Enemy/Warrior/Animations/Idle_Montage.Idle_Montage"))

(event Input|KeyboardEvents|LeftAlt
  (params (Key :type Key%20Structure :default "None"))
  ;[0.05098 0.05098 0.05098] UseWeapon
  ;;[0.05098 0.05098 0.05098] AltAttacks
  (:Pressed
    (Variables|Default|Setholding true))
  (:Released
    (Variables|Default|Setholding false)))

(fn ConstructionScript
  (switch Utilities|FlowControl|Switch|SwitchonEnemyEnum (Variables|Default|GetEnemyType)
    (:NewEnumerator0
      (bind _returnvalue (AddComponent|AddChildActorComponent false))
      (ChildActorComponent|SetChildActorClass _returnvalue "/Game/Weapons/Axe/BP_Axe.BP_Axe_C")
      (Transformation|AttachComponentToComponent _returnvalue (Variables|Default|GetBackAxe) "None" "SnapToTarget" "SnapToTarget" "SnapToTarget" true)
      (bind _asbp_axe (Utilities|Casting|CastToBP_Axe (Variables|/Script/Engine.ChildActorComponent|GetChildActor _returnvalue)))
      (Variables|Default|SetAxeRef _asbp_axe)
      (Variables|Default|SetcanAttack true))
    (:NewEnumerator1
      (bind _returnvalue_2 (AddComponent|AddChildActorComponent false))
      (ChildActorComponent|SetChildActorClass _returnvalue_2 "/Game/Weapons/Bow/BP_Bow.BP_Bow_C")
      (Transformation|AttachComponentToComponent _returnvalue_2 (Variables|Default|GetBackBow) "None" "SnapToTarget" "SnapToTarget" "SnapToTarget" true)
      (bind _asbp_bow (Utilities|Casting|CastToBP_Bow (Variables|/Script/Engine.ChildActorComponent|GetChildActor _returnvalue_2)))
      (Variables|Default|SetBowRef _asbp_bow)
      (Variables|Default|SetcanAttack true))))

(fn CheckUpperBody
  (if (> (Math|Vector|VectorLength (Variables|/Script/Engine.MovementComponent|GetVelocity (Variables|Character|GetCharacterMovement))) 1e+02)
    (Variables|Default|SetUpperBody true)
    (else
      (Variables|Default|SetUpperBody false))))

(fn RunInjuredTimer
  (params (DeltaTime :type Float%20%28double-precision%29))
  (if (Variables|Default|GetisInjured)
    (bind _output_get (Variables|Default|SetinjuredTimer (+ (Variables|Default|GetinjuredTimer) DeltaTime)))
    (if (>= _output_get (Variables|Default|GetinjuredTimerMax))
      (Variables|Default|SetisInjured false)
      (Variables|Default|SetinjuredTimer 0.0))))

(fn Attack
  (switch Utilities|FlowControl|Switch|SwitchonEnemyEnum (Variables|Default|GetEnemyType)
    (:NewEnumerator0
      (CallFunction|MeleeCall))
    (:NewEnumerator1
      (CallFunction|BowCall)))
  (return (Variables|Default|GetattackAnimLength)))

(fn GetCanMove
  (return (and (Variables|Default|GetcanMove) (Variables|Default|GetcanAttack))))

(fn GetGlobalTension
  (bind _asbp_third_person_character (Utilities|Casting|CastToBP_ThirdPersonCharacter (Game|GetPlayerCharacter 0)))
  (return (Variables|/Game/ThirdPerson/Blueprints/BP_ThirdPersonCharacter.BP_ThirdPersonCharacter_C|GettensionLevel _asbp_third_person_character)))

(fn GetIsInjured
  (return (Variables|Default|GetisInjured)))

(fn GetPatrolRoute
  (return (Variables|Default|GetPatrolRoute)))

(fn GetState
  (return (Utilities|Enum|ByteToEnumTensionEnum (Class|BlackboardComponent|GetValueasEnum (AI|GetBlackboard (AI|GetAIController self)) (Utilities|Name|MakeLiteralName "State")))))

(fn GetStatus
  (return (Variables|/Game/ThirdPerson/Blueprints/BPC_Stats.BPC_Stats_C|GetisDead (Variables|Default|GetBPC_Stats))))

(fn GetTarget
  (bind _asbp_aicontroller_general (Utilities|Casting|CastToBP_AIController_General (Pawn|GetController)))
  (Utilities|IsValid (Variables|/Game/AI/BP_AIController_General.BP_AIController_General_C|GetattackTarget _asbp_aicontroller_general)
    (:Is%20Valid
      (return (Variables|/Game/AI/BP_AIController_General.BP_AIController_General_C|GetattackTarget _asbp_aicontroller_general)))))

(fn GetType
  (return (Variables|Default|GetEnemyType)))

(fn IsArmed
  (return (Variables|Default|GetIsArmed_0)))

(fn IsDead
  (return (Variables|/Game/ThirdPerson/Blueprints/BPC_Stats.BPC_Stats_C|GetisDead (Variables|Default|GetBPC_Stats))))

(fn StealthAssassination
  (Rendering|SetVisibility (Variables|Default|GetAssassinatePrompt) false false)
  (Rendering|SetVisibility (Variables|Default|GetHealthBar) true false)
  (CallFunction|ReceiveAssassination)
  (return (Transformation|GetWorldLocation (Variables|Default|GetAssassinREF)) (Transformation|GetActorRotation)))