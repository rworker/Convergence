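; Boss enemy character with combo melee, a rock throw and random charge or leap specials, reporting attack completion through dispatchers.
; Melee montages use timer-driven limb sphere traces; the charge knocks down on contact and stuns the boss on obstacles.
; The leap follows a five-point Motion Warping arc toward the AI controller's target, ending in AoE knockdown.
; Damage updates a health bar, plays hit reactions when interruptible, and ragdolls on death.
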(event Custom|CheckRunCharge
  (bind _returnvalue (Transformation|GetActorLocation))
  (if (Variables|Default|Getcharging)
    (Variables|Default|SetdamageOnContact true)
    (Pawn|Input|AddMovementInput (Variables|Default|GetChargeDirection) 1.0 false)
    (bind (_outhit _returnvalue_2) (Collision|CapsuleTraceByChannel _returnvalue _returnvalue 1e+02 6e+01 "TraceTypeQuery1" false 0 "Persistent"))
    (if _returnvalue_2
      (Utilities|Casting|CastToBP_ThirdPersonCharacter (.HitActor (Collision|BreakHitResult _outhit))
        (:then
          (Development|PrintString "knockdown")
          (Variables|Default|Setcharging false :!label _label)
          (Animation|Montage|PlayMontage (Variables|Character|GetMesh) "/Game/Characters/Enemy/Boss/Root/Anims/Run_To_Stop_Montage.Run_To_Stop_Montage"
            (:OnCompleted
              _)
            (:OnInterrupted
              _))
          (Variables|Default|SetdamageOnContact false)
          (Animation|Montage|PlayMontage (Variables|Character|GetMesh) "/Game/Characters/Enemy/Boss/Root/Anims/Mutant_Flexing_Muscles_Montage.Mutant_Flexing_Muscles_Montage"
            (:OnCompleted
              _)
            (:OnInterrupted
              _))
          (Utilities|FlowControl|Delay 1.0)
          (Variables|Default|SetcanBeInterrupted true))
        (:CastFailed
          (Utilities|Casting|CastToBP_ArrowFly (.HitActor (Collision|BreakHitResult _outhit))
            (:CastFailed
              (Development|PrintString "Stunned")
              (Variables|Default|Setcharging false)
              (Variables|Default|SetisStunned true)
              (Components|Movement|StopMovementImmediately (Variables|Character|GetCharacterMovement))
              (Animation|Montage|PlayMontage (Variables|Character|GetMesh) "/Game/Characters/Enemy/Boss/Root/Anims/Standing_React_Large_From_Front_Montage.Standing_React_Large_From_Front_Montage"
                (:OnCompleted
                  _)
                (:OnInterrupted
                  _))
              (Variables|Default|SetdamageOnContact false)
              (Utilities|FlowControl|Delay 8.0)
              (Variables|Default|SetisStunned false)
              (Variables|Default|SetcanBeInterrupted true)))))
      (Default|CallOnFinishSpecialAttack)
      (elif (>= (Math|Vector|Distance(Vector) (Variables|Default|GetStartingChargeLocation) (Transformation|GetActorLocation)) 2e+03)
        (goto _label)))))

(event Custom|ChooseSpecialAttack
  (switch int (Math|Random|RandomInteger 2)
    (:0
      (CallFunction|ChargeAttack))
    (:1
      (CallFunction|JumpAttack))))

(event Custom|ResetAttackTrace
  (Utilities|FlowControl|DoOnce false) ; enters at Reset
)

(event Custom|BasicAttackLoop
  (bind _attackindex (Variables|Default|GetAttackIndex))
  (bind _lightanims (Variables|Default|GetLightAnims))
  (bind _output (Utilities|Array|Get(acopy) _lightanims _attackindex))
  (Utilities|FlowControl|DoOnce false :!label _label
    (:Completed
      (Utilities|FlowControl|Delay 0.1)
      (Variables|Default|SetattackAnimLength (Animation|GetPlayLength _output))
      (Variables|Default|SetCurrentAttackMontage _output)
      (Variables|Default|SetTraceIndex (Variables|Default|GetAttackIndex))
      (Animation|Montage|PlayMontage (Variables|Character|GetMesh) _output
        (:then
          (Math|Integer|IncrementInt (Variables|Default|GetAttackIndex)
            (:%20%20
              (goto _label Reset))))))))

(event Custom|StartAttackTrace
  (bind _returnvalue (Utilities|Time|SetTimerbyEvent (delegate Custom|AttackTraceLoop) 0.001 true))
  (Variables|Default|SetAttackTraceTimer _returnvalue))

(event Custom|AttackTraceLoop
  (bind (_start _end _radius) (CallFunction|SetTraceParameters (Variables|Default|GetTraceIndex)))
  (bind (_outhit _returnvalue) (Collision|SphereTraceByChannel _start _end _radius "TraceTypeQuery1" false 0 "ForOneFrame" true "(R=1.000000,G=0.000000,B=0.000000,A=1.000000)" "(R=0.000000,G=1.000000,B=0.000000,A=1.000000)" 0.2))
  (if _returnvalue
    (if (Actor|ActorHasTag (.HitActor (Collision|BreakHitResult _outhit)) "Damageable")
      (Utilities|FlowControl|DoOnce false
        (:Completed
          (Niagara|SpawnSystematLocation "/Game/Weapons/Arrow/ArrowBloodBurst.ArrowBloodBurst" (.ImpactPoint (Collision|BreakHitResult _outhit)))
          (Game|Damage|ApplyDamage (.HitActor (Collision|BreakHitResult _outhit)) (Variables|Default|GetAttackDamage) 0 self))))))

(event Custom|JumpAttack
  (bind _returnvalue (Transformation|GetActorLocation))
  (bind _returnvalue_2 (Transformation|GetActorLocation))
  (bind (_x _y _z) (Math|Vector|BreakVector _returnvalue))
  (bind (_x_2 _y_2 _z_2) (Math|Vector|BreakVector _returnvalue_2))
  (bind _returnvalue_3 (- _z_2 139.0))
  (bind _returnvalue_4 (Math|Vector|MakeVector _x_2 _y_2 _returnvalue_3))
  (Variables|Default|SetcanBeInterrupted false)
  (Animation|Montage|PlayMontage (Variables|Character|GetMesh) "/Game/Characters/Enemy/Boss/Root/Anims/Zombie_Scream_Montage.Zombie_Scream_Montage"
    (:OnCompleted
      _)
    (:OnInterrupted
      _))
  (Components|Movement|StopMovementImmediately (Variables|Character|GetCharacterMovement))
  (Pawn|Components|CharacterMovement|SetMovementMode (Variables|Character|GetCharacterMovement) "MOVE_Flying" 0)
  (for _index (range 1 5)
    (Development|PrintString (Utilities|String|ToString(Vector) (Transformation|GetActorLocation)))
    (bind _vector (CallFunction|GetJumpWarpLocation _index 7e+02))
    (Class|MotionWarpingComponent|AddorUpdateWarpTarget (Variables|Default|GetMotionWarping) (Utilities|Struct|MakeMotionWarpingTarget (Utilities|String|StringToName (Utilities|String|ToString(Integer) (Class|KismetSystemLibrary|MakeLiteralInteger _index))) _vector "0.000000,0.000000,0.000000" 0 "None" false)))
  (bind _target (CallFunction|GetTarget))
  (Transformation|SetActorRotation (Math|Rotator|FindLookatRotation (Math|Vector|MakeVector _x _y (- _z 139.0)) (Math|Vector|MakeVector (.X (Math|Vector|BreakVector (Transformation|GetActorLocation _target))) (.Y (Math|Vector|BreakVector (Transformation|GetActorLocation _target))) (- (.Z (Math|Vector|BreakVector (Transformation|GetActorLocation _target))) 92.0))))
  (bind _notifyname (Animation|Montage|PlayMontage (Variables|Character|GetMesh) "/Game/Characters/Enemy/Boss/Root/Anims/Mutant_Jump_Attack_Montage.Mutant_Jump_Attack_Montage")
    (:OnCompleted
      (Pawn|Components|CharacterMovement|SetMovementMode (Variables|Character|GetCharacterMovement) "MOVE_Walking" 0)
      (Variables|Default|SetcanBeInterrupted true)
      (Default|CallOnFinishSpecialAttack))
    (:OnNotifyBegin
      (if (== _notifyname "AoE")
        (bind (_outhits _returnvalue_5) (Collision|MultiSphereTraceByChannel _returnvalue_4 _returnvalue_4 3.5e+02 "TraceTypeQuery1" false 0 "ForDuration"))
        (if _returnvalue_5
          (bind _array_element (Utilities|Array|ForEachLoopwithBreak _outhits)
            (:LoopBody
              (Class|BPICombat|FallDown(Message) (.HitActor (Collision|BreakHitResult _array_element)) (* (Math|Vector|Normalize (.Normal (Collision|BreakHitResult _array_element))) -1.0) (.Location (Collision|BreakHitResult _array_element)) self 1e+02 3e+01))))))))

(event Custom|StopAttackTrace
  (Utilities|Time|ClearandInvalidateTimerbyHandle (Variables|Default|GetAttackTraceTimer))
  (CallFunction|ResetAttackTrace))

(event Custom|ChargeAttack
  (bind _returnvalue (Transformation|GetActorLocation))
  (bind (_x _y _z) (Math|Vector|BreakVector _returnvalue))
  (Variables|Default|SetcanBeInterrupted false)
  (Animation|Montage|PlayMontage (Variables|Character|GetMesh) "/Game/Characters/Enemy/Boss/Root/Anims/Standing_Taunt_Battlecry_Montage.Standing_Taunt_Battlecry_Montage"
    (:OnCompleted
      _)
    (:OnInterrupted
      _))
  (CallFunction|SetMovementSpeed 2e+03)
  (bind _target (CallFunction|GetTarget))
  (Variables|Default|SetChargeDirection (Math|Vector|Normalize (- (Transformation|GetActorLocation _target) _returnvalue)))
  (Transformation|SetActorRotation (Math|Rotator|FindLookatRotation (Math|Vector|MakeVector _x _y (- _z 139.0)) (Math|Vector|MakeVector (.X (Math|Vector|BreakVector (Transformation|GetActorLocation _target))) (.Y (Math|Vector|BreakVector (Transformation|GetActorLocation _target))) (- (.Z (Math|Vector|BreakVector (Transformation|GetActorLocation _target))) 92.0))))
  (Variables|Default|SetStartingChargeLocation (Transformation|GetActorLocation))
  (Variables|Default|Setcharging true))

(event Custom|RockSpawn
  (Variables|Default|GetRock
    (:then)
    (:else
      (bind _returnvalue (Game|SpawnActorfromClass "/Game/Weapons/Rock/BP_Rock.BP_Rock_C" (Transformation|GetWorldTransform (Variables|Character|GetMesh)) "Undefined" "MultiplyWithRoot" 0 self))
      (Variables|Default|SetRock _returnvalue)
      (Transformation|AttachComponentToComponent (Variables|/Script/Engine.Actor|GetRootComponent _returnvalue) (Variables|Default|GetRightHand) "None" "SnapToTarget" "SnapToTarget" "KeepWorld" true))))

(event Custom|ExecuteThrowAttack
  (bind _righthand (Variables|Default|GetRightHand))
  (bind _returnvalue (Transformation|GetWorldLocation _righthand))
  (bind _target (CallFunction|GetTarget))
  (Variables|Default|SetcanBeInterrupted false)
  (AI|SetFocus (AI|GetAIController self) _target)
  (bind _notifyname (Animation|Montage|PlayMontage (Variables|Character|GetMesh) "/Game/Characters/Enemy/Boss/Root/Anims/Throw_Object_Montage.Throw_Object_Montage")
    (:OnNotifyBegin
      (if (== _notifyname "PickUp")
        (CallFunction|RockSpawn))
      (if (== _notifyname "Throw")
        (CallFunction|GetTarget)
        (bind _tossvelocity (Class|GameplayStatics|BlueprintSuggestProjectileVelocity _returnvalue (Transformation|GetActorLocation (Game|GetPlayerCharacter 0)) (Variables|Default|GetThrowStrength) 0.0 "DoNotTrace" 0.0 false false))
        (Game|SpawnActorfromClass "/Game/Weapons/Rock/BP_RockFly.BP_RockFly_C" (Math|Transform|MakeTransform _returnvalue (Math|Rotator|MakeRotfromX _tossvelocity) "1.000000,1.000000,1.000000") "Undefined" "MultiplyWithRoot" 0 (Variables|Default|GetThrowStrength) self)
        (bind _rock (Variables|Default|GetRock)
          (:then
            (Actor|DestroyActor _rock))
          (:else
            _))
        (Utilities|FlowControl|Delay 3.0)
        (Default|CallOnFinishThrowAttack)))))

(event Custom|BasicAttack
  (Variables|Default|SetisAttacking true)
  (CallFunction|BasicAttackLoop))

(event Custom|BasicAttackCombo
  (if (Variables|Default|GetsaveAttack)
    (Variables|Default|SetsaveAttack false)
    (CallFunction|BasicAttackLoop)))

(event Custom|StopCombo
  (Variables|Default|SetisAttacking false)
  (Variables|Default|SetAttackIndex 0)
  (Variables|Default|SetisHeavy false)
  (Utilities|FlowControl|Delay 0.5)
  (Default|CallOnFinishedAttackLocal)
  (Animation|StopAnimMontage (Variables|Default|GetCurrentAttackMontage)))

(event EventBeginPlay
  (|CallParentFunction) ; This node is disabled and will not be called.\nDrag off pins to build functionality.
)

(event EventThrowAttack
  (CallFunction|ExecuteThrowAttack))

(event EventTick
  (params (DeltaSeconds :type Float%20%28single-precision%29))
  (bind _returnvalue (AI|GetBlackboard 0))
  (bind _returnvalue_2 (Utilities|Name|MakeLiteralName "TargetActor"))
  (bind _returnvalue_3 (AI|Components|Blackboard|GetValueasObject _returnvalue _returnvalue_2))
  (CallFunction|CheckRunCharge)
  (CallFunction|RunInjuredTimer DeltaSeconds)
  (Transformation|SetWorldRotation (Variables|Default|GetEnemyStats) (Math|Rotator|FindLookatRotation (Transformation|GetWorldLocation (Variables|Default|GetEnemyStats)) (Transformation|GetWorldLocation (Variables|/Script/Engine.PlayerCameraManager|GetTransformComponent (Game|GetPlayerCameraManager 0)))) false false)
  (CallFunction|CheckUpperBody)
  (CallFunction|RunInjuredTimer DeltaSeconds)
  (Utilities|IsValid _returnvalue_3
    (:Is%20Valid
      (bind _asactor (Utilities|Casting|CastToActor _returnvalue_3))
      (Class|BPAnimInterface|SetUpperBodyRotation(Message) (Components|SkeletalMesh|GetAnimInstance (Variables|Character|GetMesh)) (Math|Rotator|MakeRotator (- 3.6e+02 (.pitch (Math|Rotator|FindLookatRotation (Transformation|GetActorLocation) (Transformation|GetActorLocation _asactor)))) 0.0 0.0)))))

(event Game|Damage|EventAnyDamage
  (params (Damage :type Float%20%28single-precision%29) (DamageType :type Damage%20Type%20Object%20Reference) (InstigatedBy :type Controller%20Object%20Reference) (DamageCauser :type Actor%20Object%20Reference))
  (bind _healthui (Variables|Default|GetHealthUI))
  (bind _healthbar (Variables|/Game/UI/WB_EnemyHealth.WB_EnemyHealth_C|GetHealthBar _healthui))
  (Class|NavMovementComponent|StopActiveMovement (Variables|Character|GetCharacterMovement))
  (if (not (Variables|/Game/ThirdPerson/Blueprints/BPC_Stats.BPC_Stats_C|GetisDead (Variables|Default|GetBPC_Stats)))
    (if (Variables|Default|GetisInjured)
      _
      (elif (Variables|Default|GetcanBeInterrupted)
        (Variables|Default|SetisInjured true)
        (Animation|Montage|PlayMontage (Variables|Character|GetMesh) (Utilities|Array|Get(acopy) (Variables|Default|GethitAnims) (Math|Random|RandomIntegerinRange 0 (- (Utilities|Array|Length (Variables|Default|GethitAnims)) 1)))
          (:then
            _))))
    (bind (_isdead _healthpercent) (Default|DecreaseHealth (Variables|Default|GetBPC_Stats) Damage))
    (if (Widget|IsVisible _healthbar)
      _
      (else
        (Widget|SetVisibility _healthbar "Visible")))
    (Progress|SetPercent (Variables|/Game/UI/WB_EnemyHealth.WB_EnemyHealth_C|GetHealthBar (Variables|Default|GetHealthUI)) _healthpercent)
    (if _isdead
      (Utilities|FlowControl|Delay 0.2)
      (CallFunction|Die))))

(event EventDie
  (Default|CallEnemyDeath self)
  (Pawn|Components|CharacterMovement|DisableMovement (Variables|Character|GetCharacterMovement))
  (Rendering|SetVisibility (Variables|Default|GetEnemyStats) false false)
  (CallFunction|Ragdoll)
  (Collision|SetCollisionEnabled (Variables|Default|GetCapsuleComponent) "NoCollision")
  (Components|DestroyComponent (Variables|Default|GetCapsuleComponent)))

(event EventSpecialAttack
  (CallFunction|ChooseSpecialAttack))

(event EventGetStunned
  (Variables|Default|SetisInjured true)
  (Variables|Default|SetinjuredTimerMax 8.0)
  (Variables|Default|SetisStunned true))

(event Collision|EventHit
  (params (MyComp :type Primitive%20Component%20Object%20Reference) (Other :type Actor%20Object%20Reference) (OtherComp :type Primitive%20Component%20Object%20Reference) (bSelfMoved :type Boolean) (HitLocation :type Vector :default "0, 0, 0") (HitNormal :type Vector :default "0, 0, 0") (NormalImpulse :type Vector :default "0, 0, 0") (Hit :type Hit%20Result%20Structure%20%28by%20ref%29))
  (if (Variables|Default|GetdamageOnContact)
    (if (Utilities|DoesObjectImplementInterface Other "/Game/ThirdPerson/Blueprints/BPI_Combat.BPI_Combat_C")
      (Class|BPICombat|FallDown(Message) Other (* (.Normal (Collision|BreakHitResult Hit)) "-1.000000,-1.000000,1.000000") HitLocation self 7e+01 3e+01))))

(fn ConstructionScript
  (|CallParentFunction))

(fn Attack
  (CallFunction|BasicAttack)
  (return 0.0))

(fn LightAttack)

(fn HeavyAttack)

(fn GetTarget
  (bind _asbp_aicontroller_boss (Utilities|Casting|CastToBP_AIController_Boss (AI|GetAIController self)))
  (return (Variables|/Game/AI/Boss/BP_AIController_Boss.BP_AIController_Boss_C|GetattackTarget _asbp_aicontroller_boss)))

(fn RunInjuredTimer
  (params (DeltaTime :type Float%20%28double-precision%29))
  (if (Variables|Default|GetisInjured)
    (bind _output_get (Variables|Default|SetinjuredTimer (+ (Variables|Default|GetinjuredTimer) DeltaTime)))
    (if (>= _output_get (Variables|Default|GetinjuredTimerMax))
      (Variables|Default|SetisInjured false)
      (Variables|Default|SetinjuredTimer 0.0)
      (Variables|Default|SetisStunned false)
      (Variables|Default|SetcanBeInterrupted true))))

(fn GetJumpWarpLocation
  (params (Section :type Integer) (MaxHeight :type Float%20%28double-precision%29))
  (bind _returnvalue (Transformation|GetActorLocation))
  (bind _returnvalue_2 (* MaxHeight 0.5))
  (bind (_x _y _z) (Math|Vector|BreakVector _returnvalue))
  (bind _returnvalue_3 (- _z 139.0))
  (bind _returnvalue_4 (Math|Vector|MakeVector _x _y _returnvalue_3))
  (bind _target (CallFunction|GetTarget))
  (switch int Section
    (:1
      (Variables|Default|SetJumpHeight _returnvalue_2))
    (:2
      (Variables|Default|SetJumpHeight MaxHeight))
    (:3
      (Variables|Default|SetJumpHeight MaxHeight))
    (:4
      (Variables|Default|SetJumpHeight _returnvalue_2))
    (:5
      (Variables|Default|SetJumpHeight (.Z (Math|Vector|BreakVector (* (/ (* (Math|Vector|GetUnitDirection(Vector) _returnvalue_4 (Math|Vector|MakeVector (.X (Math|Vector|BreakVector (Transformation|GetActorLocation _target))) (.Y (Math|Vector|BreakVector (Transformation|GetActorLocation _target))) (- (.Z (Math|Vector|BreakVector (Transformation|GetActorLocation _target))) 92.0))) (- (Math|Vector|Distance(Vector) (Math|Vector|MakeVector (.X (Math|Vector|BreakVector (Transformation|GetActorLocation _target))) (.Y (Math|Vector|BreakVector (Transformation|GetActorLocation _target))) (- (.Z (Math|Vector|BreakVector (Transformation|GetActorLocation _target))) 92.0)) _returnvalue_4) 2e+02)) 5) Section))))))
  (return (+ (Math|Vector|MakeVector (.X (Math|Vector|BreakVector (* (/ (* (Math|Vector|GetUnitDirection(Vector) _returnvalue_4 (Math|Vector|MakeVector (.X (Math|Vector|BreakVector (Transformation|GetActorLocation _target))) (.Y (Math|Vector|BreakVector (Transformation|GetActorLocation _target))) (- (.Z (Math|Vector|BreakVector (Transformation|GetActorLocation _target))) 92.0))) (- (Math|Vector|Distance(Vector) (Math|Vector|MakeVector (.X (Math|Vector|BreakVector (Transformation|GetActorLocation _target))) (.Y (Math|Vector|BreakVector (Transformation|GetActorLocation _target))) (- (.Z (Math|Vector|BreakVector (Transformation|GetActorLocation _target))) 92.0)) _returnvalue_4) 2e+02)) 5) Section))) (.Y (Math|Vector|BreakVector (* (/ (* (Math|Vector|GetUnitDirection(Vector) _returnvalue_4 (Math|Vector|MakeVector (.X (Math|Vector|BreakVector (Transformation|GetActorLocation _target))) (.Y (Math|Vector|BreakVector (Transformation|GetActorLocation _target))) (- (.Z (Math|Vector|BreakVector (Transformation|GetActorLocation _target))) 92.0))) (- (Math|Vector|Distance(Vector) (Math|Vector|MakeVector (.X (Math|Vector|BreakVector (Transformation|GetActorLocation _target))) (.Y (Math|Vector|BreakVector (Transformation|GetActorLocation _target))) (- (.Z (Math|Vector|BreakVector (Transformation|GetActorLocation _target))) 92.0)) _returnvalue_4) 2e+02)) 5) Section))) (Variables|Default|GetJumpHeight)) _returnvalue_4)))

(fn CheckUpperBody
  (if (Variables|Default|GetcanBeInterrupted)
    (if (> (Math|Vector|VectorLength (Variables|/Script/Engine.MovementComponent|GetVelocity (Variables|Character|GetCharacterMovement))) 1e+02)
      (if (Variables|Default|GetisInjured)
        (Variables|Default|SetUpperBody false :!label _label)
        (else
          (Variables|Default|SetUpperBody true)))
      (else
        (goto _label)))
    (else
      (goto _label))))

(fn SetTraceParameters
  (params (Index :type Integer))
  (return (Utilities|Select :Index Index :Option%200 (Transformation|GetWorldLocation (Variables|Default|GetRightHand)) :Option%201 (Transformation|GetWorldLocation (Variables|Default|GetLeftHand)) :Option%202 (Transformation|GetWorldLocation (Variables|Default|GetRightFoot)) :Option%203 (Transformation|GetWorldLocation (Variables|Default|GetRightHand))) (Utilities|Select :Index Index :Option%200 (Transformation|GetWorldLocation (Variables|Default|GetRightArm)) :Option%201 (Transformation|GetWorldLocation (Variables|Default|GetLeftArm)) :Option%202 (Transformation|GetWorldLocation (Variables|Default|GetRightCalf)) :Option%203 (Transformation|GetWorldLocation (Variables|Default|GetRightArm))) (Utilities|Select :Index Index :Option%200 3e+01 :Option%201 3e+01 :Option%202 3e+01 :Option%203 3e+01)))