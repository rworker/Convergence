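; Boss enemy character with montage-driven melee combos, a health bar widget and interruptible hit reactions.
; Melee hits use timer-driven limb sphere traces; specials randomly pick a rock throw, leap or charge.
; The leap sets five motion-warping targets for an arc ending in an AoE knockdown; the charge stuns the boss on hitting obstacles.
; RemoteActivation sets Active, but the logic starting AI and boss combat UI is disconnected.
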(event Custom|CheckRunCharge
  (bind _returnvalue (Transformation|GetActorForwardVector))
  (bind _returnvalue_2 (Transformation|GetActorLocation))
  (bind _returnvalue_3 (* _returnvalue 5e+01))
  (bind _returnvalue_4 (+ _returnvalue_2 _returnvalue_3))
  ;[0.05098 0.05098 0.05098] ChargeAttackCheck
  (if (Variables|Default|Getcharging)
    (Variables|Default|SetdamageOnContact true)
    (Pawn|Input|AddMovementInput (Variables|Default|GetChargeDirection) 1.0 false)
    (bind (_outhit _returnvalue_5) (Collision|CapsuleTraceByChannel _returnvalue_4 (- _returnvalue_4 "0.000000,0.000000,30.000000") 7e+01 6e+01 "TraceTypeQuery1" false 0 "None"))
    (if _returnvalue_5
      (Utilities|Casting|CastToBP_ThirdPersonCharacter (.HitActor (Collision|BreakHitResult _outhit))
        (:then
          (Development|PrintString "knockdown")
          (Variables|Default|Setcharging false :!label _label)
          (Animation|Montage|PlayMontage (Variables|Character|GetMesh) "/Game/Characters/Enemy/Boss/Root/Anims/Run_To_Stop_Montage.Run_To_Stop_Montage"
            (:OnCompleted
              _)
            (:OnInterrupted
              _))
          (Variables|Default|SetdamageOnContact false)
          (Animation|Montage|PlayMontage (Variables|Character|GetMesh) "/Game/Characters/Enemy/Boss/Root/Anims/Mutant_Flexing_Muscles_Montage.Mutant_Flexing_Muscles_Montage"
            (:OnCompleted
              _)
            (:OnInterrupted
              _))
          (Utilities|FlowControl|Delay 1.0)
          (Variables|Default|SetcanBeInterrupted true))
        (:CastFailed
          (Utilities|Casting|CastToBP_ArrowFly (.HitActor (Collision|BreakHitResult _outhit))
            (:CastFailed
              (Development|PrintString "Stunned")
              (Variables|Default|Setcharging false)
              (Variables|Default|SetisStunned true)
              (Components|Movement|StopMovementImmediately (Variables|Character|GetCharacterMovement))
              (Animation|Montage|PlayMontage (Variables|Character|GetMesh) "/Game/Characters/Enemy/Boss/Root/Anims/Standing_React_Large_From_Front_Montage.Standing_React_Large_From_Front_Montage"
                (:OnCompleted
                  _)
                (:OnInterrupted
                  _))
              (Variables|Default|SetdamageOnContact false)
              (Utilities|FlowControl|Delay 8.0)
              (Variables|Default|SetisStunned false)
              (Variables|Default|SetcanBeInterrupted true)))))
      (Default|CallOnFinishSpecialAttack)
      (elif (>= (Math|Vector|Distance(Vector) (Variables|Default|GetStartingChargeLocation) (Transformation|GetActorLocation)) 2e+03)
        (goto _label)))))

(event Custom|ChooseSpecialAttack
  ;[0.05098 0.05098 0.05098] SpecialAttackCalls
  (switch int (Math|Random|RandomInteger 3)
    (:0
      (CallFunction|ThrowAttack))
    (:1
      (CallFunction|JumpAttack))
    (:2
      (CallFunction|ChargeAttack))))

(event Custom|CheckActive
  ;[0.05098 0.05098 0.05098] Activate/Deactivate
)

(event Custom|ResetAttackTrace
  ;[0.05098 0.05098 0.05098] AttackTrace
  (Utilities|FlowControl|DoOnce false) ; enters at Reset
)

(event Custom|DeactivateBossCombat
  ;[0.05098 0.05098 0.05098] Activate/Deactivate
  (bind _bosshealth (Variables|Default|GetBossHealth)
    (:then
      (Widget|RemovefromParent _bosshealth))
    (:else)))

(event Custom|RemoteActivation
  ;[0.05098 0.05098 0.05098] Activate/Deactivate
  (Variables|Default|SetActive? true))

(event Custom|BasicAttackLoop
  (bind _attackindex (Variables|Default|GetAttackIndex))
  (bind _lightanims (Variables|Default|GetLightAnims))
  (bind _output (Utilities|Array|Get(acopy) _lightanims _attackindex))
  ;[0.05098 0.05098 0.05098] BasicAttack
  (Utilities|FlowControl|DoOnce false :!label _label
    (:Completed
      (Utilities|FlowControl|Delay 0.1)
      (Variables|Default|SetattackAnimLength (Animation|GetPlayLength _output))
      (Variables|Default|SetCurrentAttackMontage _output)
      (Variables|Default|SetTraceIndex (Variables|Default|GetAttackIndex))
      (Animation|Montage|PlayMontage (Variables|Character|GetMesh) _output
        (:then
          (Math|Integer|IncrementInt (Variables|Default|GetAttackIndex)
            (:%20%20
              (goto _label Reset))))))))

(event Custom|StartAttackTrace
  ;[0.05098 0.05098 0.05098] AttackTrace
  (bind _returnvalue (Utilities|Time|SetTimerbyEvent (delegate Custom|AttackTraceLoop) 0.001 true))
  (Variables|Default|SetAttackTraceTimer _returnvalue))

(event Custom|AttackTraceLoop
  ;[0.05098 0.05098 0.05098] AttackTrace
  (bind (_start _end _radius) (CallFunction|SetTraceParameters (Variables|Default|GetTraceIndex)))
  (bind (_outhit _returnvalue) (Collision|SphereTraceByChannel _start _end _radius "TraceTypeQuery1" false 0 "ForOneFrame" true "(R=1.000000,G=0.000000,B=0.000000,A=1.000000)" "(R=0.000000,G=1.000000,B=0.000000,A=1.000000)" 0.2))
  (if _returnvalue
    (if (Actor|ActorHasTag (.HitActor (Collision|BreakHitResult _outhit)) "Damageable")
      (Utilities|FlowControl|DoOnce false
        (:Completed
          (Niagara|SpawnSystematLocation "/Game/Weapons/Arrow/ArrowBloodBurst.ArrowBloodBurst" (.ImpactPoint (Collision|BreakHitResult _outhit)))
          (Game|Damage|ApplyDamage (.HitActor (Collision|BreakHitResult _outhit)) (Variables|Default|GetAttackDamage) 0 self))))))

(event Custom|JumpAttack
  (bind _returnvalue (Transformation|GetActorLocation))
  (bind (_x _y _z) (Math|Vector|BreakVector _returnvalue))
  (bind _returnvalue_2 (- _z 139.0))
  (bind _returnvalue_3 (Math|Vector|MakeVector _x _y _returnvalue_2))
  ;[0.05098 0.05098 0.05098] JumpAttack
  (bind _target (CallFunction|GetTarget))
  (Variables|Default|SetcanBeInterrupted false)
  (AI|SetFocus (AI|GetAIController self) _target)
  (Animation|Montage|PlayMontage (Variables|Character|GetMesh) "/Game/Characters/Enemy/Boss/Root/Anims/Zombie_Scream_Montage.Zombie_Scream_Montage"
    (:OnCompleted
      _)
    (:OnInterrupted
      _))
  (Components|Movement|StopMovementImmediately (Variables|Character|GetCharacterMovement))
  (Pawn|Components|CharacterMovement|SetMovementMode (Variables|Character|GetCharacterMovement) "MOVE_Flying" 0)
  (for _index (range 1 5)
    (Development|PrintString (Utilities|String|ToString(Vector) (Transformation|GetActorLocation)))
    (bind _vector (CallFunction|GetJumpWarpLocation _index 7e+02))
    (Class|MotionWarpingComponent|AddorUpdateWarpTarget (Variables|Default|GetMotionWarping) (Utilities|Struct|MakeMotionWarpingTarget (Utilities|String|StringToName (Utilities|String|ToString(Integer) (Class|KismetSystemLibrary|MakeLiteralInteger _index))) _vector "0.000000,0.000000,0.000000" 0 "None" false)))
  (bind _notifyname (Animation|Montage|PlayMontage (Variables|Character|GetMesh) "/Game/Characters/Enemy/Boss/Root/Anims/Mutant_Jump_Attack_Montage.Mutant_Jump_Attack_Montage")
    (:OnCompleted
      (Pawn|Components|CharacterMovement|SetMovementMode (Variables|Character|GetCharacterMovement) "MOVE_Walking" 0)
      (Variables|Default|SetcanBeInterrupted true)
      (Default|CallOnFinishSpecialAttack))
    (:OnNotifyBegin
      (if (== _notifyname "AoE")
        (Effects|SpawnEmitteratLocation "/Game/Particles/InfinityBladeEffects/Effects/FX_Skill_Leap/P_Skill_Leap_Fire_Velocity_Suction.P_Skill_Leap_Fire_Velocity_Suction" _returnvalue_3 (Transformation|GetActorRotation))
        (bind (_outhits _returnvalue_4) (Collision|MultiSphereTraceByChannel _returnvalue_3 _returnvalue_3 4e+02 "TraceTypeQuery1" false 0 "ForDuration"))
        (if _returnvalue_4
          (bind _array_element (Utilities|Array|ForEachLoopwithBreak _outhits)
            (:LoopBody
              (Class|BPICombat|FallDown(Message) (.HitActor (Collision|BreakHitResult _array_element)) (* (Math|Vector|Normalize (.Normal (Collision|BreakHitResult _array_element))) -1.0) (.Location (Collision|BreakHitResult _array_element)) self 1e+02 3e+01))))))))

(event Custom|StopAttackTrace
  ;[0.05098 0.05098 0.05098] AttackTrace
  (Utilities|Time|ClearandInvalidateTimerbyHandle (Variables|Default|GetAttackTraceTimer))
  (CallFunction|ResetAttackTrace))

(event Custom|ChargeAttack
  (bind _returnvalue (Transformation|GetActorLocation))
  (bind (_x _y _z) (Math|Vector|BreakVector _returnvalue))
  ;[0.05098 0.05098 0.05098] ChargeAttack
  (bind _target (CallFunction|GetTarget))
  (bind (_outhit _returnvalue_2) (Collision|LineTraceByChannel (Transformation|GetWorldLocation (Variables|Default|GetLineTraceStart)) (Transformation|GetActorLocation _target) "TraceTypeQuery1" false 0 "None"))
  (if _returnvalue_2
    (if (Utilities|DoesObjectImplementInterface (.HitActor (Collision|BreakHitResult _outhit)) "/Game/ThirdPerson/Blueprints/BPI_Combat.BPI_Combat_C")
      (Variables|Default|SetcanBeInterrupted false :!label _label)
      (AI|ClearFocus (AI|GetAIController self))
      (Animation|Montage|PlayMontage (Variables|Character|GetMesh) "/Game/Characters/Enemy/Boss/Root/Anims/Standing_Taunt_Battlecry_Montage.Standing_Taunt_Battlecry_Montage"
        (:OnCompleted
          _)
        (:OnInterrupted
          _))
      (CallFunction|SetMovementSpeed 2e+03)
      (bind _target_2 (CallFunction|GetTarget))
      (Variables|Default|SetChargeDirection (Math|Vector|Normalize (- (Transformation|GetActorLocation _target_2) _returnvalue)))
      (Transformation|SetActorRotation (Math|Rotator|FindLookatRotation (Math|Vector|MakeVector _x _y (- _z 139.0)) (Math|Vector|MakeVector (.X (Math|Vector|BreakVector (Transformation|GetActorLocation _target_2))) (.Y (Math|Vector|BreakVector (Transformation|GetActorLocation _target_2))) (- (.Z (Math|Vector|BreakVector (Transformation|GetActorLocation _target_2))) 92.0))))
      (Variables|Default|SetStartingChargeLocation (Transformation|GetActorLocation))
      (Variables|Default|Setcharging true)
      (else
        (switch int (Math|Random|RandomInteger 2)
          (:0
            (CallFunction|ThrowAttack))
          (:1
            (CallFunction|JumpAttack)))))
    (else
      (goto _label))))

(event Custom|RockSpawn
  ;[0.05098 0.05098 0.05098] ThrowAttack
  (Variables|Default|GetRock
    (:then)
    (:else
      (bind _returnvalue (Game|SpawnActorfromClass "/Game/Weapons/Rock/BP_Rock.BP_Rock_C" (Transformation|GetWorldTransform (Variables|Character|GetMesh)) "Undefined" "MultiplyWithRoot" 0 self))
      (Variables|Default|SetRock _returnvalue)
      (Transformation|AttachComponentToComponent (Variables|/Script/Engine.Actor|GetRootComponent _returnvalue) (Variables|Default|GetRightHand) "None" "SnapToTarget" "SnapToTarget" "KeepWorld" true))))

(event Custom|ExecuteThrowAttack
  (bind _righthand (Variables|Default|GetRightHand))
  (bind _returnvalue (Transformation|GetWorldLocation _righthand))
  ;[0.05098 0.05098 0.05098] ThrowAttack
  (bind _target (CallFunction|GetTarget))
  (Variables|Default|SetcanBeInterrupted false)
  (AI|SetFocus (AI|GetAIController self) _target)
  (bind _notifyname (Animation|Montage|PlayMontage (Variables|Character|GetMesh) "/Game/Characters/Enemy/Boss/Root/Anims/Throw_Object_Montage.Throw_Object_Montage")
    (:OnNotifyBegin
      (if (== _notifyname "PickUp")
        (CallFunction|RockSpawn))
      (if (== _notifyname "Throw")
        (CallFunction|GetTarget)
        (bind _tossvelocity (Class|GameplayStatics|BlueprintSuggestProjectileVelocity _returnvalue (Transformation|GetActorLocation (Game|GetPlayerCharacter 0)) (Variables|Default|GetThrowStrength) 0.0 "DoNotTrace" 0.0 false false))
        (Game|SpawnActorfromClass "/Game/Weapons/Rock/BP_RockFly.BP_RockFly_C" (Math|Transform|MakeTransform _returnvalue (Math|Rotator|MakeRotfromX _tossvelocity) "1.000000,1.000000,1.000000") "Undefined" "MultiplyWithRoot" 0 (Variables|Default|GetThrowStrength) self)
        (bind _rock (Variables|Default|GetRock)
          (:then
            (Actor|DestroyActor _rock))
          (:else
            _))
        (Utilities|FlowControl|Delay 3.0)
        (AI|ClearFocus (AI|GetAIController self))
        (Default|CallOnFinishThrowAttack)
        (Default|CallOnFinishSpecialAttack)))))

(event Custom|BasicAttack
  ;[0.05098 0.05098 0.05098] BasicAttack
  (Variables|Default|SetisAttacking true)
  (CallFunction|BasicAttackLoop))

(event Custom|BasicAttackCombo
  ;[0.05098 0.05098 0.05098] BasicAttack
  (if (Variables|Default|GetsaveAttack)
    (Variables|Default|SetsaveAttack false)
    (CallFunction|BasicAttackLoop)))

(event Custom|StopCombo
  ;[0.05098 0.05098 0.05098] BasicAttack
  (Variables|Default|SetisAttacking false)
  (Variables|Default|SetAttackIndex 0)
  (Variables|Default|SetisHeavy false)
  (Utilities|FlowControl|Delay 0.5)
  (Default|CallOnFinishedAttackLocal)
  (Animation|StopAnimMontage (Variables|Default|GetCurrentAttackMontage)))

(event Custom|ActivateBossCombat
  (bind _returnvalue (Game|GetPlayerCharacter 0))
  ;[0.05098 0.05098 0.05098] Activate/Deactivate
  (Utilities|IsValid (Variables|Default|GetBossHealth)
    (:Is%20Valid
      _)
    (:Is%20Not%20Valid
      (bind _returnvalue_2 (UserInterface|CreateWidget "/Game/UI/WB_BossHealth.WB_BossHealth_C" (Game|GetPlayerController 0)))
      (Variables|Default|SetBossHealth _returnvalue_2)))
  (bind _healthpercent (Default|GetCurrentHealth (Variables|Default|GetBPC_Stats)))
  (Progress|SetPercent (Variables|/Game/UI/WB_BossHealth.WB_BossHealth_C|GetHealthBar (Variables|Default|GetBossHealth)) _healthpercent)
  (UserInterface|Viewport|AddtoViewport (Variables|Default|GetBossHealth) 0)
  (bind _asbp_third_person_character (Utilities|Casting|CastToBP_ThirdPersonCharacter _returnvalue))
  (Default|TriggerCombat _asbp_third_person_character "/Game/Audio/Assets/Sounds/Music/Ice_BossBattle01.Ice_BossBattle01")
  (Default|PlayDialogue :self (Variables|/Game/ThirdPerson/Blueprints/BP_ThirdPersonCharacter.BP_ThirdPersonCharacter_C|GetDialogueSystem _asbp_third_person_character) :Conversation "/Game/Dialogue/Conversations/Conversation7.Conversation7" :Location (Transformation|GetActorLocation _returnvalue)))

(event EventBeginPlay)

(event EventThrowAttack
  ;[0.05098 0.05098 0.05098] SpecialAttackCalls
  (CallFunction|ExecuteThrowAttack))

(event EventTick
  (params (DeltaSeconds :type Float%20%28single-precision%29))
  (bind _returnvalue (AI|GetBlackboard 0))
  (bind _returnvalue_2 (Utilities|Name|MakeLiteralName "TargetActor"))
  (bind _returnvalue_3 (AI|Components|Blackboard|GetValueasObject _returnvalue _returnvalue_2))
  ;[0.05098 0.05098 0.05098] Tick
  (CallFunction|CheckActive)
  (if (Variables|Default|GetActive?)
    (CallFunction|CheckRunCharge)
    (CallFunction|RunInjuredTimer DeltaSeconds)
    (CallFunction|CheckUpperBody)
    (Utilities|IsValid _returnvalue_3
      (:Is%20Valid
        (bind _asactor (Utilities|Casting|CastToActor _returnvalue_3))
        (Class|BPAnimInterface|SetUpperBodyRotation(Message) (Components|SkeletalMesh|GetAnimInstance (Variables|Character|GetMesh)) (Math|Rotator|MakeRotator (- 3.6e+02 (.pitch (Math|Rotator|FindLookatRotation (Transformation|GetActorLocation) (Transformation|GetActorLocation _asactor)))) 0.0 0.0))))))

(event Game|Damage|EventAnyDamage
  (params (Damage :type Float%20%28single-precision%29) (DamageType :type Damage%20Type%20Object%20Reference) (InstigatedBy :type Controller%20Object%20Reference) (DamageCauser :type Actor%20Object%20Reference))
  ;[0.05098 0.05098 0.05098] Damage
  (Class|NavMovementComponent|StopActiveMovement (Variables|Character|GetCharacterMovement))
  (if (not (Variables|/Game/ThirdPerson/Blueprints/BPC_Stats.BPC_Stats_C|GetisDead (Variables|Default|GetBPC_Stats)))
    (if (Variables|Default|GetisInjured)
      _
      (elif (Variables|Default|GetcanBeInterrupted)
        (Variables|Default|SetisInjured true)
        (Animation|Montage|PlayMontage (Variables|Character|GetMesh) (Utilities|Array|Get(acopy) (Variables|Default|GethitAnims) (Math|Random|RandomIntegerinRange 0 (- (Utilities|Array|Length (Variables|Default|GethitAnims)) 1)))
          (:then
            _))))
    (bind (_isdead _healthpercent) (Default|DecreaseHealth (Variables|Default|GetBPC_Stats) Damage))
    (Progress|SetPercent (Variables|/Game/UI/WB_BossHealth.WB_BossHealth_C|GetHealthBar (Variables|Default|GetBossHealth)) _healthpercent)
    (if _isdead
      (Utilities|FlowControl|Delay 0.2)
      (CallFunction|Die))))

(event EventDie
  (bind _bpc_stats (Variables|Default|GetBPC_Stats))
  ;[0.05098 0.05098 0.05098] Die
  (if (> (Variables|/Game/ThirdPerson/Blueprints/BPC_Stats.BPC_Stats_C|GetCurrentHealth _bpc_stats) 0.0)
    (Default|DecreaseHealth _bpc_stats 1e+03))
  (Default|CallEnemyDeath self)
  (Variables|Default|SetActive? false)
  (Pawn|Components|CharacterMovement|DisableMovement (Variables|Character|GetCharacterMovement))
  (Rendering|SetVisibility (Variables|Default|GetEnemyStats) false false)
  (Collision|SetCollisionEnabled (Variables|Default|GetCapsuleComponent) "NoCollision")
  (Components|DestroyComponent (Variables|Default|GetCapsuleComponent))
  (bind _asbp_third_person_character (Utilities|Casting|CastToBP_ThirdPersonCharacter (Game|GetPlayerCharacter 0)))
  (Default|EndCombat _asbp_third_person_character))

(event EventSpecialAttack
  ;[0.05098 0.05098 0.05098] SpecialAttackCalls
  (CallFunction|ChooseSpecialAttack))

(event EventGetStunned
  ;[0.05098 0.05098 0.05098] SpecialAttackCalls
)

(event Collision|EventHit
  (params (MyComp :type Primitive%20Component%20Object%20Reference) (Other :type Actor%20Object%20Reference) (OtherComp :type Primitive%20Component%20Object%20Reference) (bSelfMoved :type Boolean) (HitLocation :type Vector :default "0, 0, 0") (HitNormal :type Vector :default "0, 0, 0") (NormalImpulse :type Vector :default "0, 0, 0") (Hit :type Hit%20Result%20Structure%20%28by%20ref%29))
  ;[0.05098 0.05098 0.05098] ChargeAttack
  (if (Variables|Default|GetdamageOnContact)
    (if (Utilities|DoesObjectImplementInterface Other "/Game/ThirdPerson/Blueprints/BPI_Combat.BPI_Combat_C")
      (Class|BPICombat|FallDown(Message) Other (* (.Normal (Collision|BreakHitResult Hit)) "-1.000000,-1.000000,1.000000") HitLocation self 7e+01 3e+01))))

(fn ConstructionScript
  (|CallParentFunction))

(fn Attack
  (CallFunction|BasicAttack)
  (return 0.0))

(fn LightAttack)

(fn HeavyAttack)

(fn GetTarget
  (bind _asbp_aicontroller_boss (Utilities|Casting|CastToBP_AIController_Boss (AI|GetAIController self)))
  (return (Variables|/Game/AI/Boss/BP_AIController_Boss.BP_AIController_Boss_C|GetattackTarget _asbp_aicontroller_boss)))

(fn RunInjuredTimer
  (params (DeltaTime :type Float%20%28double-precision%29))
  (if (Variables|Default|GetisInjured)
    (bind _output_get (Variables|Default|SetinjuredTimer (+ (Variables|Default|GetinjuredTimer) DeltaTime)))
    (if (>= _output_get (Variables|Default|GetinjuredTimerMax))
      (Variables|Default|SetisInjured false)
      (Variables|Default|SetinjuredTimer 0.0)
      (Variables|Default|SetisStunned false))))

(fn GetJumpWarpLocation
  (params (Section :type Integer) (MaxHeight :type Float%20%28double-precision%29))
  (bind _returnvalue (Transformation|GetActorLocation))
  (bind _returnvalue_2 (* MaxHeight 0.5))
  (bind (_x _y _z) (Math|Vector|BreakVector _returnvalue))
  (bind _returnvalue_3 (- _z 139.0))
  (bind _returnvalue_4 (Math|Vector|MakeVector _x _y _returnvalue_3))
  (bind _target (CallFunction|GetTarget))
  (switch int Section
    (:1
      (Variables|Default|SetJumpHeight _returnvalue_2))
    (:2
      (Variables|Default|SetJumpHeight MaxHeight))
    (:3
      (Variables|Default|SetJumpHeight MaxHeight))
    (:4
      (Variables|Default|SetJumpHeight _returnvalue_2))
    (:5
      (Variables|Default|SetJumpHeight (.Z (Math|Vector|BreakVector (* (/ (* (Math|Vector|GetUnitDirection(Vector) _returnvalue_4 (Math|Vector|MakeVector (.X (Math|Vector|BreakVector (Transformation|GetActorLocation _target))) (.Y (Math|Vector|BreakVector (Transformation|GetActorLocation _target))) (- (.Z (Math|Vector|BreakVector (Transformation|GetActorLocation _target))) 92.0))) (- (Math|Vector|Distance(Vector) (Math|Vector|MakeVector (.X (Math|Vector|BreakVector (Transformation|GetActorLocation _target))) (.Y (Math|Vector|BreakVector (Transformation|GetActorLocation _target))) (- (.Z (Math|Vector|BreakVector (Transformation|GetActorLocation _target))) 92.0)) _returnvalue_4) 2e+02)) 5) Section))))))
  (return (+ (Math|Vector|MakeVector (.X (Math|Vector|BreakVector (* (/ (* (Math|Vector|GetUnitDirection(Vector) _returnvalue_4 (Math|Vector|MakeVector (.X (Math|Vector|BreakVector (Transformation|GetActorLocation _target))) (.Y (Math|Vector|BreakVector (Transformation|GetActorLocation _target))) (- (.Z (Math|Vector|BreakVector (Transformation|GetActorLocation _target))) 92.0))) (- (Math|Vector|Distance(Vector) (Math|Vector|MakeVector (.X (Math|Vector|BreakVector (Transformation|GetActorLocation _target))) (.Y (Math|Vector|BreakVector (Transformation|GetActorLocation _target))) (- (.Z (Math|Vector|BreakVector (Transformation|GetActorLocation _target))) 92.0)) _returnvalue_4) 2e+02)) 5) Section))) (.Y (Math|Vector|BreakVector (* (/ (* (Math|Vector|GetUnitDirection(Vector) _returnvalue_4 (Math|Vector|MakeVector (.X (Math|Vector|BreakVector (Transformation|GetActorLocation _target))) (.Y (Math|Vector|BreakVector (Transformation|GetActorLocation _target))) (- (.Z (Math|Vector|BreakVector (Transformation|GetActorLocation _target))) 92.0))) (- (Math|Vector|Distance(Vector) (Math|Vector|MakeVector (.X (Math|Vector|BreakVector (Transformation|GetActorLocation _target))) (.Y (Math|Vector|BreakVector (Transformation|GetActorLocation _target))) (- (.Z (Math|Vector|BreakVector (Transformation|GetActorLocation _target))) 92.0)) _returnvalue_4) 2e+02)) 5) Section))) (Variables|Default|GetJumpHeight)) _returnvalue_4)))

(fn CheckUpperBody
  (if (Variables|Default|GetcanBeInterrupted)
    (if (> (Math|Vector|VectorLength (Variables|/Script/Engine.MovementComponent|GetVelocity (Variables|Character|GetCharacterMovement))) 1e+02)
      (if (Variables|Default|GetisInjured)
        (Variables|Default|SetUpperBody false :!label _label)
        (else
          (Variables|Default|SetUpperBody true)))
      (else
        (goto _label)))
    (else
      (goto _label))))

(fn SetTraceParameters
  (params (Index :type Integer))
  (return (Utilities|Select :Index Index :Option%200 (Transformation|GetWorldLocation (Variables|Default|GetRightHand)) :Option%201 (Transformation|GetWorldLocation (Variables|Default|GetLeftHand)) :Option%202 (Transformation|GetWorldLocation (Variables|Default|GetRightFoot)) :Option%203 (Transformation|GetWorldLocation (Variables|Default|GetRightHand))) (Utilities|Select :Index Index :Option%200 (Transformation|GetWorldLocation (Variables|Default|GetRightArm)) :Option%201 (Transformation|GetWorldLocation (Variables|Default|GetLeftArm)) :Option%202 (Transformation|GetWorldLocation (Variables|Default|GetRightCalf)) :Option%203 (Transformation|GetWorldLocation (Variables|Default|GetRightArm))) (Utilities|Select :Index Index :Option%200 3e+01 :Option%201 3e+01 :Option%202 3e+01 :Option%203 3e+01)))