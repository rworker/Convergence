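; AI controller for the boss that runs BT_AI_Boss on BeginPlay and sets the player character as the TargetActor blackboard key.
; The perception update event does nothing, as its sight, hearing and damage dispatch is disconnected, so perception does not drive targeting.
; Leftover detection, forgot-actor and search logic would write target and location keys and switch pawn states, but nothing in this graph calls it.
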(event OnTargetPerceptionUpdated(AIPerception)
  (params (Actor :type Actor%20Object%20Reference) (Stimulus :type AI%20Stimulus%20Structure)))

(event EventBeginPlay
  (AI|RunBehaviorTree "/Game/AI/Boss/BT_AI_Boss.BT_AI_Boss")
  (AI|Components|Blackboard|SetValueasObject (AI|GetBlackboard 0) (Utilities|Name|MakeLiteralName "TargetActor") (Game|GetPlayerCharacter 0)))

(event EventTick
  (params (DeltaSeconds :type Float%20%28single-precision%29)))

(fn ConstructionScript)

(fn SightDetection
  (params (Actor :type Actor%20Object%20Reference) (Stimulus :type AI%20Stimulus%20Structure))
  (Utilities|Array|AddUnique (Variables|Default|GetKnownSeenActors) Actor)
  (bind _returnvalue (Class|AIPerceptionSystem|GetSenseClassforStimulus Stimulus))
  (if (== _returnvalue "/Script/AIModule.AISense_Sight")
    (if (.bSuccessfullySensed (Utilities|Struct|BreakAIStimulus Stimulus))
      (bind _isdead (Class|BPICombat|IsDead(Message) Actor))
      (if (not _isdead)
        (AI|Components|Blackboard|SetValueasObject (AI|GetBlackboard 0) (Utilities|Name|MakeLiteralName "TargetActor") Actor)
        (bind _asbp_ai (Utilities|Casting|CastToBP_AI (Pawn|GetControlledPawn)))
        (Default|CallOnFoundTarget _asbp_ai _asbp_ai Actor)
        (Variables|Default|SetattackTarget Actor))
      (else
        (AI|Components|Blackboard|SetValueasObject (AI|GetBlackboard 0) (Utilities|Name|MakeLiteralName "TargetActor") 0)
        (Utilities|Casting|CastToBP_AI (Pawn|GetControlledPawn))))))

(fn HearingDetection
  (params (Actor :type Actor%20Object%20Reference) (Stimulus :type AI%20Stimulus%20Structure))
  (bind _returnvalue (Class|AIPerceptionSystem|GetSenseClassforStimulus Stimulus))
  (if (== _returnvalue "/Script/AIModule.AISense_Hearing")
    (bind _globaltension (Class|BPIAIBehaviors|GetGlobalTension(Message) (Pawn|GetControlledPawn)))
    (if (or (Utilities|Enum|Equal(Enum) _globaltension "NewEnumerator0") (Utilities|Enum|Equal(Enum) _globaltension "NewEnumerator1"))
      (AI|Components|Blackboard|SetValueasVector (AI|GetBlackboard 0) (Utilities|Name|MakeLiteralName "InvestigationLocation") (.StimulusLocation (Utilities|Struct|BreakAIStimulus Stimulus)))
      (Class|BPICombat|SetState(Message) (Pawn|GetControlledPawn) "NewEnumerator1"))))

(fn DamageDetection
  (params (Actor :type Actor%20Object%20Reference) (Stimulus :type AI%20Stimulus%20Structure))
  (bind _returnvalue (Class|AIPerceptionSystem|GetSenseClassforStimulus Stimulus))
  (if (== _returnvalue "/Script/AIModule.AISense_Damage")
    (bind _globaltension (Class|BPIAIBehaviors|GetGlobalTension(Message) (Pawn|GetControlledPawn)))
    (if (or (Utilities|Enum|Equal(Enum) _globaltension "NewEnumerator0") (Utilities|Enum|Equal(Enum) _globaltension "NewEnumerator1"))
      (AI|Components|Blackboard|SetValueasVector (AI|GetBlackboard 0) (Utilities|Name|MakeLiteralName "InvestigationLocation") (.StimulusLocation (Utilities|Struct|BreakAIStimulus Stimulus)))
      (Class|BPICombat|SetState(Message) (Pawn|GetControlledPawn) "NewEnumerator1"))))

(fn HandleForgotActor
  (params (Actor :type Actor%20Object%20Reference))
  (Development|PrintString "Hello")
  (Utilities|Array|RemoveItem (Variables|Default|GetKnownSeenActors) Actor)
  (if (== Actor (Variables|Default|GetattackTarget))
    (AI|Components|Blackboard|SetValueasObject (AI|GetBlackboard 0) (Utilities|Name|MakeLiteralName "TargetActor") 0)
    (bind _isdead (Class|BPICombat|IsDead(Message) Actor))
    (if _isdead
      (Class|BPICombat|SetState(Message) (Pawn|GetControlledPawn) "NewEnumerator0")
      (else
        (AI|Components|Blackboard|SetValueasVector (AI|GetBlackboard 0) (Utilities|Name|MakeLiteralName "SearchLocation") (Transformation|GetActorLocation Actor))
        (Class|BPICombat|SetState(Message) (Pawn|GetControlledPawn) "NewEnumerator3")))))