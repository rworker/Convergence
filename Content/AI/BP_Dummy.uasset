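; BP_Dummy is an enemy dummy character that takes damage, arrow hits and stealth assassinations.
; BPCStats tracks health for a camera-facing health bar, while damage triggers random hit montages and knockback along the player's forward vector.
; Arrows attach to the nearest bone before applying damage; assassination plays a paired victim montage whose notify zeroes health.
; Death ragdolls the mesh, hides the bar and disables the capsule and assassination radius.
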(event Custom|Ragdoll
  (Physics|SetSimulatePhysics (Variables|Character|GetMesh) true))

(event Custom|ReceiveAssassination
  (Animation|Montage|PlayMontage (Variables|Character|GetMesh) "/Game/Characters/Mannequins/Animations/Quinn/Assassination/Paired_Knife_Stealth_KidneyAndNeck_Vic_Montage.Paired_Knife_Stealth_KidneyAndNeck_Vic_Montage"
    (:OnBlendOut
      (CallFunction|Die))
    (:OnNotifyBegin
      (bind _healthpercent (Default|InstaKill (Variables|Default|GetBPC_Stats)))
      (Progress|SetPercent (Variables|/Game/UI/WB_EnemyHealth.WB_EnemyHealth_C|GetHealthBar (Variables|Default|GetHealthUI)) _healthpercent))))

(event Custom|Die
  (Rendering|SetVisibility (Variables|Default|GetHealthBar) false false)
  (CallFunction|Ragdoll)
  (Components|Activation|SetActive (Variables|Default|GetAssassination%20Radius) false false)
  (Collision|SetCollisionEnabled (Variables|Collision|GetCapsuleComponent) "NoCollision")
  (Components|DestroyComponent (Variables|Collision|GetCapsuleComponent)))

(event EventBeginPlay
  (bind _aswb_enemy_health (Utilities|Casting|CastToWB_EnemyHealth (UserInterface|GetWidget (Variables|Default|GetHealthBar))))
  (bind _output_get (Variables|Default|SetHealthUI _aswb_enemy_health))
  (bind _healthpercent (Default|GetCurrentHealth (Variables|Default|GetBPC_Stats)))
  (Progress|SetPercent (Variables|/Game/UI/WB_EnemyHealth.WB_EnemyHealth_C|GetHealthBar _output_get) _healthpercent))

(event Collision|EventActorBeginOverlap
  (params (OtherActor :type Actor%20Object%20Reference)))

(event EventTick
  (params (DeltaSeconds :type Float%20%28single-precision%29))
  (Transformation|SetWorldRotation (Variables|Default|GetHealthBar) (Math|Rotator|FindLookatRotation (Transformation|GetWorldLocation (Variables|Default|GetHealthBar)) (Transformation|GetWorldLocation (Variables|/Script/Engine.PlayerCameraManager|GetTransformComponent (Game|GetPlayerCameraManager 0)))) false false))

(event Game|Damage|EventAnyDamage
  (params (Damage :type Float%20%28single-precision%29) (DamageType :type Damage%20Type%20Object%20Reference) (InstigatedBy :type Controller%20Object%20Reference) (DamageCauser :type Actor%20Object%20Reference))
  (bind _healthbar (Variables|Default|GetHealthBar))
  (if (not (Variables|/Game/ThirdPerson/Blueprints/BPC_Stats.BPC_Stats_C|GetisDead (Variables|Default|GetBPC_Stats)))
    (Animation|PlayAnimMontage (Utilities|Array|Get(acopy) (Variables|Default|GethitAnims) (Math|Random|RandomIntegerinRange 0 (- (Utilities|Array|Length (Variables|Default|GethitAnims)) 1))) 1.0 "None")
    (bind _asbp_third_person_character (Utilities|Casting|CastToBP_ThirdPersonCharacter (Game|GetPlayerCharacter 0)))
    (Character|LaunchCharacter (* (Math|Vector|GetForwardVector (Transformation|GetActorRotation _asbp_third_person_character)) 7e+02) false false)
    (bind (_isdead _healthpercent) (Default|DecreaseHealth (Variables|Default|GetBPC_Stats) Damage))
    (if (Rendering|IsVisible _healthbar)
      _
      (else
        (Rendering|SetVisibility _healthbar true false)))
    (Progress|SetPercent (Variables|/Game/UI/WB_EnemyHealth.WB_EnemyHealth_C|GetHealthBar (Variables|Default|GetHealthUI)) _healthpercent)
    (if _isdead
      (Utilities|FlowControl|Delay 0.2)
      (CallFunction|Die))))

(event EventArrowDamage
  (params (Damage :type Float%20%28double-precision%29) (Arrow :type BP%20Arrow%20Fly%20Object%20Reference) (HitLocation :type Vector :default "0, 0, 0") (Shooter :type Pawn%20Object%20Reference))
  (Transformation|AttachComponentToComponent Arrow (Variables|Character|GetMesh) (.ReturnValue (Class|SkinnedMeshComponent|FindClosestBoneK2 (Variables|Character|GetMesh) HitLocation 0.0)) "SnapToTarget" "KeepWorld" "KeepWorld" true)
  (Game|Damage|ApplyDamage self Damage 0 0))

(fn ConstructionScript)

(fn GetState
  (return "NewEnumerator0"))

(fn GetStatus
  (return (Variables|/Game/ThirdPerson/Blueprints/BPC_Stats.BPC_Stats_C|GetisDead (Variables|Default|GetBPC_Stats))))

(fn GetType
  (return "NewEnumerator0"))

(fn IsDead
  (return false))

(fn StealthAssassination
  (Rendering|SetVisibility (Variables|Default|GetHealthBar) true false)
  (CallFunction|ReceiveAssassination)
  (return (Transformation|GetWorldLocation (Variables|Default|GetAssassinREF)) (Transformation|GetActorRotation)))