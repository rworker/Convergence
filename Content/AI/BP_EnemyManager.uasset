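; Coordinates a group of BP_AI enemies, binding to their events at BeginPlay to share targets, set player tension and control attack turns.
; A found target goes to blackboards lacking one, and enemy tensions resolve by priority into the player's TensionLevel.
; Tick gives one random in-range enemy the canAttack blackboard flag as a single attack token.
; Leaving range or death frees the token immediately; finishing an attack frees it after a delay.
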(event Custom|CheckEnemyTensions
  (Variables|Default|SetloopBroken false)
  (bind _array_element (Utilities|Array|ForEachLoopwithBreak (Variables|Default|GetEnemies) :!label _label)
    (:LoopBody
      (if (not (Utilities|Enum|Equal(Enum) (Variables|/Game/AI/BP_AI.BP_AI_C|GetTension _array_element) (Variables|/Game/ThirdPerson/Blueprints/BP_ThirdPersonCharacter.BP_ThirdPersonCharacter_C|GettensionLevel (Variables|Default|GetPlayer))))
        (if (Utilities|Enum|Equal(Enum) (Variables|/Game/AI/BP_AI.BP_AI_C|GetTension _array_element) "NewEnumerator2")
          (Variables|/Game/ThirdPerson/Blueprints/BP_ThirdPersonCharacter.BP_ThirdPersonCharacter_C|SettensionLevel (Variables|Default|GetPlayer) "NewEnumerator2")
          (Variables|Default|SetloopBroken true)
          (goto _label Break))))
    (:Completed
      (if (not (Variables|Default|GetloopBroken))
        (bind _array_element_2 (Utilities|Array|ForEachLoopwithBreak (Variables|Default|GetEnemies) :!label _label_2)
          (:LoopBody
            (if (Utilities|Enum|Equal(Enum) (Variables|/Game/AI/BP_AI.BP_AI_C|GetTension _array_element_2) "NewEnumerator3")
              (Variables|/Game/ThirdPerson/Blueprints/BP_ThirdPersonCharacter.BP_ThirdPersonCharacter_C|SettensionLevel (Variables|Default|GetPlayer) "NewEnumerator3")
              (Variables|Default|SetloopBroken true)
              (goto _label_2 Break)))
          (:Completed
            (if (not (Variables|Default|GetloopBroken))
              (bind _array_element_3 (Utilities|Array|ForEachLoopwithBreak (Variables|Default|GetEnemies) :!label _label_3)
                (:LoopBody
                  (if (Utilities|Enum|Equal(Enum) (Variables|/Game/AI/BP_AI.BP_AI_C|GetTension _array_element_3) "NewEnumerator1")
                    (Variables|/Game/ThirdPerson/Blueprints/BP_ThirdPersonCharacter.BP_ThirdPersonCharacter_C|SettensionLevel (Variables|Default|GetPlayer) "NewEnumerator1")
                    (Variables|Default|SetloopBroken true)
                    (goto _label_3 Break)))
                (:Completed
                  (if (not (Variables|Default|GetloopBroken))
                    (Variables|/Game/ThirdPerson/Blueprints/BP_ThirdPersonCharacter.BP_ThirdPersonCharacter_C|SettensionLevel (Variables|Default|GetPlayer) "NewEnumerator0")))))))))))

(event Custom|SendTarget
  (params (ChaseTarget :type Object%20Object%20Reference))
  (bind _returnvalue (Utilities|Name|MakeLiteralName "TargetActor"))
  (bind _array_element (Utilities|Array|ForEachLoopwithBreak (Variables|Default|GetEnemies))
    (:LoopBody
      (if (== (AI|Components|Blackboard|GetValueasObject (AI|GetBlackboard _array_element) _returnvalue) 0)
        (AI|Components|Blackboard|SetValueasObject (AI|GetBlackboard _array_element) _returnvalue ChaseTarget)))))

(event Custom|CloseEnemiesList
  (params (Enemy :type BP%20AI%20Object%20Reference) (inRange :type Boolean))
  (bind _returnvalue (AI|GetBlackboard Enemy))
  (bind _returnvalue_2 (Utilities|Name|MakeLiteralName "canAttack"))
  (bind _closeenemies (Variables|Default|GetCloseEnemies))
  (if inRange
    (if (not (Utilities|Array|ContainsItem _closeenemies Enemy))
      (Utilities|Array|Add _closeenemies Enemy))
    (else
      (Utilities|Array|RemoveItem (Variables|Default|GetCloseEnemies) Enemy)
      (if (== (ScalableFloat|GetValueasBool _returnvalue _returnvalue_2) true)
        (AI|Components|Blackboard|SetValueasBool _returnvalue _returnvalue_2 false)
        (Variables|Default|SetisAttacking false)))))

(event Custom|DeactivateActiveEnemy
  (params (Enemy :type BP%20AI%20Object%20Reference))
  (AI|Components|Blackboard|SetValueasBool (AI|GetBlackboard Enemy) (Utilities|Name|MakeLiteralName "canAttack") false)
  (Utilities|FlowControl|Delay 2.0)
  (Variables|Default|SetisAttacking false))

(event Custom|RemoveEnemy
  (params (Enemy :type Actor%20Object%20Reference))
  (bind _returnvalue (AI|GetBlackboard Enemy))
  (bind _returnvalue_2 (Utilities|Name|MakeLiteralName "canAttack"))
  (bind _asbp_ai (Utilities|Casting|CastToBP_AI Enemy))
  (Utilities|Array|RemoveItem (Variables|Default|GetCloseEnemies) _asbp_ai)
  (Utilities|Array|RemoveItem (Variables|Default|GetEnemies) _asbp_ai)
  (if (== (ScalableFloat|GetValueasBool _returnvalue _returnvalue_2) true)
    (AI|Components|Blackboard|SetValueasBool _returnvalue _returnvalue_2 false)
    (Variables|Default|SetisAttacking false)))

(event EventBeginPlay
  (bind _asbp_third_person_character (Utilities|Casting|CastToBP_ThirdPersonCharacter (Game|GetPlayerCharacter 0)))
  (Variables|Default|SetPlayer _asbp_third_person_character)
  (for _array_element (Variables|Default|GetEnemies)
    (EventDispatchers|BindEventtoUpdatedTension _array_element (delegate Custom|CheckEnemyTensions))
    (EventDispatchers|BindEventtoShareTarget _array_element (delegate Custom|SendTarget))
    (EventDispatchers|BindEventtoNotifyinAttackRange _array_element (delegate Custom|CloseEnemiesList))
    (EventDispatchers|BindEventtoOnFinishedAttackGlobal _array_element (delegate Custom|DeactivateActiveEnemy))
    (EventDispatchers|BindEventtoEnemyDeath _array_element (delegate Custom|RemoveEnemy))))

(event Collision|EventActorBeginOverlap
  (params (OtherActor :type Actor%20Object%20Reference)))

(event EventTick
  (params (DeltaSeconds :type Float%20%28single-precision%29))
  (bind _closeenemies (Variables|Default|GetCloseEnemies))
  (bind _returnvalue (Utilities|Array|Length _closeenemies))
  (Development|PrintString (Utilities|String|ToString(Integer) _returnvalue))
  (if (not (Variables|Default|GetisAttacking))
    (if (>= _returnvalue 1)
      (Variables|Default|SetActiveEnemy (.OutItem (Utilities|Array|Random (Variables|Default|GetCloseEnemies))))
      (AI|Components|Blackboard|SetValueasBool (AI|GetBlackboard (Variables|Default|GetActiveEnemy)) (Utilities|Name|MakeLiteralName "canAttack") true)
      (Development|PrintString "t")
      (Variables|Default|SetisAttacking true)
      (else
        (Variables|Default|SetActiveEnemy 0)))))

(fn ConstructionScript)