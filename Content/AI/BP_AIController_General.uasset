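; General AI controller that runs the BT_AI behavior tree and turns perception events into blackboard values and pawn state changes.
; A sense-check macro routes stimuli from living pawns to sight, hearing or damage handlers, which pick states from global tension and set investigation locations, with barks for sight and hearing.
; Sight also sets the target and starts a timer on loss; Search clears a living target and stores its last location.
; Forgotten-actor handling is disconnected.
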(event OnTargetPerceptionUpdated(AIPerception)
  (params (Actor :type Actor%20Object%20Reference) (Stimulus :type AI%20Stimulus%20Structure))
  (bind _isdead (Class|BPICombat|IsDead(Message) (Pawn|GetControlledPawn)))
  (if (not _isdead)
    (Utilities|CheckSenseClass Stimulus "/Script/AIModule.AISense_Sight"
      (:else
        (Utilities|CheckSenseClass Stimulus "/Script/AIModule.AISense_Hearing"
          (:else
            (Utilities|CheckSenseClass Stimulus "/Script/AIModule.AISense_Damage"
              (:then
                (CallFunction|DamageDetection Actor Stimulus))))
          (:then
            (CallFunction|HearingDetection Actor Stimulus))))
      (:then
        (if (not (Variables|Default|GetdisableSight?))
          (CallFunction|SightDetection Actor Stimulus))))))

(event Custom|CheckIfForgottenSeenActor
  (if (!= (Utilities|Array|Length (Variables|Default|GetKnownSeenActors)) (Utilities|Array|Length (Class|AIPerceptionComponent|GetKnownPerceivedActors (Variables|Default|GetAIPerception) "/Script/AIModule.AISense_Sight")))
    (for _array_element (Variables|Default|GetKnownSeenActors)
      (if (== (Utilities|Array|FindItem (Class|AIPerceptionComponent|GetKnownPerceivedActors (Variables|Default|GetAIPerception) "/Script/AIModule.AISense_Sight") _array_element) -1)
        (CallFunction|HandleForgotActor _array_element)))))

(event Custom|Search
  (AI|Components|Blackboard|SetValueasObject (AI|GetBlackboard 0) (Utilities|Name|MakeLiteralName "TargetActor") 0)
  (bind _asbp_ai (Utilities|Casting|CastToBP_AI (Pawn|GetControlledPawn)))
  (Default|CallOnLostTarget _asbp_ai _asbp_ai)
  (bind _attacktarget (Variables|Default|GetattackTarget)
    (:then
      (bind _isdead (Class|BPICombat|IsDead(Message) _attacktarget))
      (if _isdead
        (Class|BPICombat|SetState(Message) (Pawn|GetControlledPawn) "NewEnumerator0")
        (else
          (bind _attacktarget_2 (Variables|Default|GetattackTarget)
            (:then
              (AI|Components|Blackboard|SetValueasVector (AI|GetBlackboard 0) (Utilities|Name|MakeLiteralName "SearchLocation") (Transformation|GetActorLocation _attacktarget_2))
              (Variables|Default|SetlostTarget true)
              (Variables|Default|SetattackTarget 0))
            (:else)))))
    (:else)))

(event EventBeginPlay
  (AI|RunBehaviorTree "/Game/AI/BT_AI.BT_AI")
  (AI|Components|Blackboard|SetValueasEnum (AI|GetBlackboard 0) (Variables|Default|GetStateKeyName) (Utilities|Enum|LiteralenumTensionEnum "NewEnumerator0")))

(event EventTick
  (params (DeltaSeconds :type Float%20%28single-precision%29)))

(fn ConstructionScript)

(fn SightDetection
  (params (Actor :type Actor%20Object%20Reference) (Stimulus :type AI%20Stimulus%20Structure))
  (bind (_age _expirationage _strength _stimuluslocation _receiverlocation _tag _bsuccessfullysensed) (Utilities|Struct|BreakAIStimulus Stimulus))
  (bind _returnvalue (Pawn|GetControlledPawn))
  (bind _returnvalue_2 (Pawn|GetControlledPawn))
  (Utilities|Array|AddUnique (Variables|Default|GetKnownSeenActors) Actor)
  (bind _returnvalue_3 (Class|AIPerceptionSystem|GetSenseClassforStimulus Stimulus))
  (if (== _returnvalue_3 "/Script/AIModule.AISense_Sight")
    (if _bsuccessfullysensed
      (Variables|Default|SetcanSeeTarget true)
      (Utilities|Time|ClearandInvalidateTimerbyHandle (Variables|Default|GetLostSightTimer))
      (bind _isdead (Class|BPICombat|IsDead(Message) Actor))
      (if (not _isdead)
        (Variables|Default|SetlostTarget false)
        (AI|Components|Blackboard|SetValueasObject (AI|GetBlackboard 0) (Utilities|Name|MakeLiteralName "TargetActor") Actor)
        (bind _asbp_ai (Utilities|Casting|CastToBP_AI (Pawn|GetControlledPawn)))
        (Variables|Default|SetattackTarget Actor)
        (bind _globaltension (Class|BPIAIBehaviors|GetGlobalTension(Message) (Pawn|GetControlledPawn)))
        (if (or (Utilities|Enum|Equal(Enum) _globaltension "NewEnumerator0") (Utilities|Enum|Equal(Enum) _globaltension "NewEnumerator1"))
          (AI|Components|Blackboard|SetValueasVector (AI|GetBlackboard 0) (Utilities|Name|MakeLiteralName "InvestigationLocation") _stimuluslocation)
          (Class|BPICombat|SetState(Message) _returnvalue_2 "NewEnumerator1")
          (bind _asbp_ai_2 (Utilities|Casting|CastToBP_AI _returnvalue_2))
          (Default|HandlePlayBark _asbp_ai_2 (Variables|/Game/AI/BP_AI.BP_AI_C|GetInvestigateSightBarks _asbp_ai_2) 100)
          (else
            (Class|BPICombat|SetState(Message) _returnvalue "NewEnumerator2")
            (Utilities|Casting|CastToBP_AI _returnvalue))))
      (else
        (Variables|Default|SetcanSeeTarget false)
        (bind _returnvalue_4 (Utilities|Time|SetTimerbyEvent (EventDispatchers|CreateEvent :!event Custom|Search) 3.0))
        (Variables|Default|SetLostSightTimer _returnvalue_4)))))

(fn HearingDetection
  (params (Actor :type Actor%20Object%20Reference) (Stimulus :type AI%20Stimulus%20Structure))
  (bind _returnvalue (Pawn|GetControlledPawn))
  (bind _returnvalue_2 (Class|AIPerceptionSystem|GetSenseClassforStimulus Stimulus))
  (if (== _returnvalue_2 "/Script/AIModule.AISense_Hearing")
    (bind _globaltension (Class|BPIAIBehaviors|GetGlobalTension(Message) (Pawn|GetControlledPawn)))
    (if (or (Utilities|Enum|Equal(Enum) _globaltension "NewEnumerator0") (Utilities|Enum|Equal(Enum) _globaltension "NewEnumerator1"))
      (AI|Components|Blackboard|SetValueasVector (AI|GetBlackboard 0) (Utilities|Name|MakeLiteralName "InvestigationLocation") (.StimulusLocation (Utilities|Struct|BreakAIStimulus Stimulus)))
      (Class|BPICombat|SetState(Message) _returnvalue "NewEnumerator1")
      (bind _asbp_ai (Utilities|Casting|CastToBP_AI _returnvalue))
      (Default|HandlePlayBark _asbp_ai (Variables|/Game/AI/BP_AI.BP_AI_C|GetInvestigateHearBarks _asbp_ai) 100))))

(fn DamageDetection
  (params (Actor :type Actor%20Object%20Reference) (Stimulus :type AI%20Stimulus%20Structure))
  (bind _returnvalue (Class|AIPerceptionSystem|GetSenseClassforStimulus Stimulus))
  (if (== _returnvalue "/Script/AIModule.AISense_Damage")
    (bind _globaltension (Class|BPIAIBehaviors|GetGlobalTension(Message) (Pawn|GetControlledPawn)))
    (if (or (Utilities|Enum|Equal(Enum) _globaltension "NewEnumerator0") (Utilities|Enum|Equal(Enum) _globaltension "NewEnumerator1"))
      (AI|Components|Blackboard|SetValueasVector (AI|GetBlackboard 0) (Utilities|Name|MakeLiteralName "InvestigationLocation") (.StimulusLocation (Utilities|Struct|BreakAIStimulus Stimulus)))
      (Class|BPICombat|SetState(Message) (Pawn|GetControlledPawn) "NewEnumerator1"))))

(fn HandleForgotActor
  (params (Actor :type Actor%20Object%20Reference)))