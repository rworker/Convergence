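; BP_ArrowPickup is an arrow pickup actor that shows a prompt widget when the player character is near.
; On BeginPlay it passes its Quantity to the WB_PickupPrompt widget.
; PickupRadius overlaps with BP_ThirdPersonCharacter show the prompt only if IsRetrievable is set, and hide it when the overlap ends.
; The graph handles only the prompt, with no logic for collecting the arrows.
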(event OnComponentBeginOverlap(PickupRadius)
  (params (OverlappedComponent :type Primitive%20Component%20Object%20Reference) (OtherActor :type Actor%20Object%20Reference) (OtherComp :type Primitive%20Component%20Object%20Reference) (OtherBodyIndex :type Integer) (bFromSweep :type Boolean) (SweepResult :type Hit%20Result%20Structure%20%28by%20ref%29))
  (if (Variables|Default|GetisRetrievable)
    (Utilities|Casting|CastToBP_ThirdPersonCharacter OtherActor)
    (Rendering|SetVisibility (Variables|Default|GetPickupPrompt) true false)))

(event OnComponentEndOverlap(PickupRadius)
  (params (OverlappedComponent :type Primitive%20Component%20Object%20Reference) (OtherActor :type Actor%20Object%20Reference) (OtherComp :type Primitive%20Component%20Object%20Reference) (OtherBodyIndex :type Integer))
  (Utilities|Casting|CastToBP_ThirdPersonCharacter OtherActor)
  (Rendering|SetVisibility (Variables|Default|GetPickupPrompt) false false))

(event EventBeginPlay
  (bind _aswb_pickup_prompt (Utilities|Casting|CastToWB_PickupPrompt (UserInterface|GetUserWidgetObject (Variables|Default|GetPickupPrompt))))
  (Default|SetQuantity _aswb_pickup_prompt (Variables|Default|GetQuantity)))

(event Collision|EventActorBeginOverlap
  (params (OtherActor :type Actor%20Object%20Reference)))

(fn ConstructionScript)