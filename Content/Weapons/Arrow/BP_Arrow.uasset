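; BP_Arrow is an arrow actor, used by the player or AI, that keeps its Arrow component aimed at its owner's bow.
; On BeginPlay it casts the Instigator to the third-person character or BP_AI, caches that bow reference and sets IsEnemy.
; Each tick it sets the arrow's world rotation so its X axis points from the arrow toward a spot slightly above the bow's location.
; It contains no movement, hit or damage logic.
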(event EventBeginPlay
  (bind _instigator (Variables|Actor|GetInstigator))
  (bind _asbp_third_person_character (Utilities|Casting|CastToBP_ThirdPersonCharacter _instigator)
    (:then
      (Variables|Default|SetBow (Variables|/Game/ThirdPerson/Blueprints/BP_ThirdPersonCharacter.BP_ThirdPersonCharacter_C|GetBow _asbp_third_person_character))
      (Variables|Default|SetisEnemy false))
    (:CastFailed
      (bind _asbp_ai (Utilities|Casting|CastToBP_AI _instigator))
      (Variables|Default|SetBow%20Ref (Variables|/Game/AI/BP_AI.BP_AI_C|GetBowRef _asbp_ai))
      (Variables|Default|SetisEnemy true))))

(event Collision|EventActorBeginOverlap
  (params (OtherActor :type Actor%20Object%20Reference)))

(event EventTick
  (params (DeltaSeconds :type Float%20%28single-precision%29))
  (bind _bow (Variables|Default|GetBow))
  (bind _bow_ref (Variables|Default|GetBow%20Ref))
  (bind _arrow (Variables|Default|GetArrow))
  (bind _returnvalue (Transformation|GetWorldLocation _bow))
  (bind _returnvalue_2 (Transformation|GetActorLocation _bow_ref))
  (bind (_x _y _z) (Math|Vector|BreakVector _returnvalue))
  (bind (_x_2 _y_2 _z_2) (Math|Vector|BreakVector _returnvalue_2))
  (if (Variables|Default|GetisEnemy)
    (Transformation|SetWorldRotation _arrow (Math|Rotator|MakeRotfromX (Math|Vector|Normalize (- (Math|Vector|MakeVector _x_2 _y_2 (+ _z_2 2.0)) (Transformation|GetWorldLocation (Variables|Default|GetArrow))))) false false)
    (else
      (Transformation|SetWorldRotation _arrow (Math|Rotator|MakeRotfromX (Math|Vector|Normalize (- (Math|Vector|MakeVector _x _y (+ _z 2.0)) (Transformation|GetWorldLocation (Variables|Default|GetArrow))))) false false))))

(fn ConstructionScript)