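; Flying arrow projectile that damages combat actors or sticks into whatever else it hits, with its launch speed set in construction.
; The first valid box overlap stops it, skipping its shooter, other arrows, pickups and dead combatants.
; Combat hits send damage through BPI_Combat with blood effects and a shooter bark.
; Other hits play impact effects, report noise and make the arrow retrievable, so its pickup radius shows a prompt to the player.
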(event OnComponentBeginOverlap(Box)
  (params (OverlappedComponent :type Primitive%20Component%20Object%20Reference) (OtherActor :type Actor%20Object%20Reference) (OtherComp :type Primitive%20Component%20Object%20Reference) (OtherBodyIndex :type Integer) (bFromSweep :type Boolean) (SweepResult :type Hit%20Result%20Structure%20%28by%20ref%29))
  (bind _impactpoint (Collision|BreakHitResult SweepResult))
  (bind _returnvalue (Utilities|GetClass OtherActor))
  (bind _projectilemovement (Variables|Default|GetProjectileMovement))
  (bind _instigator (Variables|Actor|GetInstigator))
  (Development|PrintString (Utilities|GetDisplayName OtherActor))
  (if (and (!= _returnvalue "/Game/Weapons/Arrow/BP_ArrowPickup.BP_ArrowPickup_C") (!= _returnvalue "BP_ArrowFly_C"))
    (if (Utilities|DoesObjectImplementInterface OtherActor "/Game/ThirdPerson/Blueprints/BPI_Combat.BPI_Combat_C")
      (bind _isdead (Class|BPICombat|IsDead(Message) OtherActor))
      (if (not _isdead)
        (if (and (!= OtherActor self) (!= OtherActor (Variables|Actor|GetInstigator))) :!label _label
          (Utilities|FlowControl|DoOnce false
            (:Completed
              (Components|Movement|StopMovementImmediately _projectilemovement)
              (Variables|/Script/Engine.ProjectileMovementComponent|SetProjectileGravityScale _projectilemovement 0.0)
              (if (Utilities|DoesObjectImplementInterface OtherActor "/Game/ThirdPerson/Blueprints/BPI_Combat.BPI_Combat_C")
                (Class|BPICombat|ArrowDamage(Message) OtherActor (Variables|Default|GetArrowDamage) self (Transformation|GetActorLocation) (Game|GetInstigator))
                (Collision|SetCollisionEnabled (Variables|Default|GetBox) "NoCollision")
                (Audio|PlaySoundatLocation "/Game/Audio/Assorted/SW_KnifeStab.SW_KnifeStab" _impactpoint "0, 0, 0" 1.0 1.0 0.0 0 0 0 0)
                (Niagara|SpawnSystematLocation "/Game/Weapons/Arrow/ArrowBloodBurst.ArrowBloodBurst" (Transformation|GetWorldLocation (Variables|Default|GetBox)))
                (bind _asbp_third_person_character (Utilities|Casting|CastToBP_ThirdPersonCharacter _instigator)
                  (:then
                    (Default|HandlePlayBark _asbp_third_person_character (Variables|/Game/ThirdPerson/Blueprints/BP_ThirdPersonCharacter.BP_ThirdPersonCharacter_C|GetArcherBarks _asbp_third_person_character) 30))
                  (:CastFailed
                    (bind _asbp_ai (Utilities|Casting|CastToBP_AI _instigator))
                    (Default|HandlePlayBark _asbp_ai (Variables|/Game/AI/BP_AI.BP_AI_C|GetMeleeBarks _asbp_ai) 30)))
                (else
                  (Variables|Default|SetisRetrievable true)
                  (Audio|PlaySoundatLocation "/Game/Audio/Assorted/SW_ArrowImpact.SW_ArrowImpact" _impactpoint "0, 0, 0" 1.0 1.0 0.0 0 0 0 0)
                  (Transformation|AttachActorToActor 0 "None" "KeepWorld" "KeepWorld" "KeepWorld" true)
                  (Collision|SetCollisionEnabled (Variables|Default|GetBox) "NoCollision")
                  (Niagara|SpawnSystematLocation "/Game/Weapons/Arrow/ArrowBurst.ArrowBurst" (Transformation|GetWorldLocation (Variables|Default|GetBox)))
                  (Class|AISenseHearing|ReportNoiseEvent (Transformation|GetActorLocation) 1.0 self 2e+03 "None")))))))
      (else
        (goto _label)))))

(event OnComponentBeginOverlap(PickupRadius)
  (params (OverlappedComponent :type Primitive%20Component%20Object%20Reference) (OtherActor :type Actor%20Object%20Reference) (OtherComp :type Primitive%20Component%20Object%20Reference) (OtherBodyIndex :type Integer) (bFromSweep :type Boolean) (SweepResult :type Hit%20Result%20Structure%20%28by%20ref%29))
  (if (Variables|Default|GetisRetrievable)
    (Utilities|Casting|CastToBP_ThirdPersonCharacter OtherActor)
    (Rendering|SetVisibility (Variables|Default|GetPickupPrompt) true false)))

(event OnComponentEndOverlap(PickupRadius)
  (params (OverlappedComponent :type Primitive%20Component%20Object%20Reference) (OtherActor :type Actor%20Object%20Reference) (OtherComp :type Primitive%20Component%20Object%20Reference) (OtherBodyIndex :type Integer))
  (Utilities|Casting|CastToBP_ThirdPersonCharacter OtherActor)
  (Rendering|SetVisibility (Variables|Default|GetPickupPrompt) false false))

(event EventBeginPlay
  (bind _newniagarasystem (Variables|Default|GetNewNiagaraSystem))
  (Utilities|FlowControl|Delay 0.05)
  (Utilities|IsValid _newniagarasystem
    (:Is%20Valid
      (Rendering|SetVisibility _newniagarasystem true false))))

(event Collision|EventActorBeginOverlap
  (params (OtherActor :type Actor%20Object%20Reference)))

(event EventTick
  (params (DeltaSeconds :type Float%20%28single-precision%29)))

(fn ConstructionScript
  (Variables|/Script/Engine.ProjectileMovementComponent|SetInitialSpeed (Variables|Default|GetProjectileMovement) (Variables|Default|GetProjectile%20Speed)))