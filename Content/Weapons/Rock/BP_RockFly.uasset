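; BP_RockFly is a flying rock projectile that shatters on overlap and damages what it hits.
; Its first valid overlap, ignoring itself, its Instigator and other rocks, stops movement and enables physics on RockBreak.
; Chaos field strain and radial velocity break and scatter the pieces, then a debug-drawn sphere trace sends FallDownMessage with damage and force to the actor found.
; The construction script sets launch speed from ProjectileSpeed.
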(event OnComponentBeginOverlap(BreakSphereCollision)
  (params (OverlappedComponent :type Primitive%20Component%20Object%20Reference) (OtherActor :type Actor%20Object%20Reference) (OtherComp :type Primitive%20Component%20Object%20Reference) (OtherBodyIndex :type Integer) (bFromSweep :type Boolean) (SweepResult :type Hit%20Result%20Structure%20%28by%20ref%29))
  (bind _returnvalue (Transformation|GetActorLocation))
  (bind _projectilemovement (Variables|Default|GetProjectileMovement))
  (bind _fieldsystem (Variables|Default|GetFieldSystem))
  (bind _spherecollision (Variables|Default|GetSphereCollision))
  (bind _returnvalue_2 (Transformation|GetWorldLocation _spherecollision))
  (if (not (== (Utilities|GetClass OtherActor) "BP_RockFly_C"))
    (if (and (!= OtherActor self) (!= OtherActor (Variables|Actor|GetInstigator)))
      (Utilities|FlowControl|DoOnce false
        (:Completed
          (Collision|SetCollisionEnabled (Variables|Default|GetBreakSphereCollision) "NoCollision")
          (Components|Movement|StopMovementImmediately _projectilemovement)
          (Variables|/Script/Engine.ProjectileMovementComponent|SetProjectileGravityScale _projectilemovement 0.0)
          (Physics|SetSimulatePhysics (Variables|Default|GetRockBreak) true)
          (Class|FieldSystemComponent|ApplyPhysicsField _fieldsystem true "Field_ExternalClusterStrain" 0 (Field|SetRadialFalloff (Variables|Default|GetRadialFalloff) 1e+01 0.0 1.0 0.0 (Components|Sphere|GetScaledSphereRadius _spherecollision) _returnvalue_2 "Field_FallOff_None"))
          (Class|FieldSystemComponent|ApplyPhysicsField _fieldsystem true "Field_LinearVelocity" 0 (Field|SetRadialVector (Variables|Default|GetRadialVector) 3e+02 _returnvalue_2))
          (bind (_outhit _returnvalue_3) (Collision|SphereTraceByChannel _returnvalue _returnvalue 1e+02 "TraceTypeQuery1" false 0 "ForDuration"))
          (if _returnvalue_3
            (Class|BPICombat|FallDown(Message) (.HitActor (Collision|BreakHitResult _outhit)) (* (Math|Vector|Normalize (.Normal (Collision|BreakHitResult _outhit))) -1.0) (.Location (Collision|BreakHitResult _outhit)) (Variables|Actor|GetInstigator) 1e+02 3e+01)))))))

(event EventBeginPlay)

(event Collision|EventActorBeginOverlap
  (params (OtherActor :type Actor%20Object%20Reference)))

(event EventTick
  (params (DeltaSeconds :type Float%20%28single-precision%29)))

(fn ConstructionScript
  (Variables|/Script/Engine.ProjectileMovementComponent|SetInitialSpeed (Variables|Default|GetProjectileMovement) (Variables|Default|GetProjectileSpeed)))